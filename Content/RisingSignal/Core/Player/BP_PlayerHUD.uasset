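; BP_PlayerHUD creates the player's in-game interface and pause menu widgets and switches between them.
; On BeginPlay it adds both to the viewport with the pause menu hidden, and binds to the player controller's OnGamePaused event and the Continue button.
; Pausing shows the menu with cursor and UI-only input.
; Continue restores the interface and game-only input, then unpauses the game.
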(event Custom|PauseEvent
  (bind _controllerref (Variables|Default|GetControllerRef))
  (Widget|SetVisibility (Variables|Default|GetPlayerInterfaceRef) "Hidden")
  (Widget|SetVisibility (Variables|Default|GetPauseWidget) "Visible")
  (Variables|/Script/Engine.PlayerController|SetbShowMouseCursor _controllerref true)
  (Input|SetInputModeUIOnly _controllerref 0 "DoNotLock"))

(event Custom|CustomEvent_0
  (CallFunction|ClearPause))

(event EventBeginPlay
  (bind _returnvalue (UserInterface|CreateWidget "/Game/RisingSignal/Core/HUD/UI_UserHUD/Widgets/WBP_PlayerInterface.WBP_PlayerInterface_C"))
  (bind _output_get (Variables|Default|SetPlayerInterfaceRef _returnvalue))
  (UserInterface|Viewport|AddtoViewport _output_get 0)
  (bind _asbp_rsgame_player_controller (Utilities|Casting|CastToBP_RSGamePlayerController (Game|GetPlayerController 0)))
  (bind _output_get_2 (Variables|Default|SetControllerRef _asbp_rsgame_player_controller))
  (EventDispatchers|BindEventtoOnGamePaused _output_get_2 (delegate Custom|PauseEvent))
  (bind _returnvalue_2 (UserInterface|CreateWidget "/Game/RisingSignal/Core/HUD/UI_UserHUD/Widgets/WBP_GamePause.WBP_GamePause_C"))
  (bind _output_get_3 (Variables|Default|SetPauseWidget _returnvalue_2))
  (UserInterface|Viewport|AddtoViewport _output_get_3 0)
  (Widget|SetVisibility _output_get_3 "Hidden")
  (EventDispatchers|BindEventtoOnClicked (Variables|/Game/RisingSignal/Core/HUD/UI_UserHUD/Widgets/WBP_GamePause.WBP_GamePause_C|GetContinueBtn (Variables|Default|GetPauseWidget)) (delegate Custom|CustomEvent_0)))

(fn ConstructionScript)

(fn ClearPause
  (bind _controllerref (Variables|Default|GetControllerRef))
  (Widget|SetVisibility (Variables|Default|GetPlayerInterfaceRef) "Visible")
  (Widget|SetVisibility (Variables|Default|GetPauseWidget) "Hidden")
  (Variables|/Script/Engine.PlayerController|SetbShowMouseCursor _controllerref false)
  (Input|SetInputModeGameOnly _controllerref)
  (Game|SetGamePaused false))