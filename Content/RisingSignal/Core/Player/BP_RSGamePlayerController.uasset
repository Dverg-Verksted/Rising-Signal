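; Player controller that creates an ALS debug HUD, toggled with Tab and V, and manages a slot-based item inventory.
; Pickups fill the first empty InventoryObjects slot and fire a pickup dispatcher.
; Move, remove and clear functions edit that array, with remove and clear also updating widgets through the character's HUD reference.
; Item use only caches the action-bar slot and image, as its use-and-remove logic is disconnected.
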(event Custom|Use%20Item%20Event
  (params (Slot :type Integer))
  (CallFunction|ItemWasUsed Slot))

(event EventBeginPlay
  (bind _asbp_test_player_character (Utilities|Casting|CastToBP_TestPlayerCharacter (Game|GetPlayerCharacter 0))
    (:then
      (Variables|Default|SetCharacterRef _asbp_test_player_character))
    (:CastFailed
      _))
  (bind _returnvalue (UserInterface|CreateWidget "/Game/RisingSignal/Core/HUD/UI_Debug/WBP_ALS_HUD_RS.WBP_ALS_HUD_RS_C" self))
  (bind _output_get (Variables|Default|SetALS_DEBUG_HUD _returnvalue))
  (UserInterface|Viewport|AddtoViewport _output_get 0))

(event EventTick
  (params (DeltaSeconds :type Float%20%28single-precision%29)))

(event Input|KeyboardEvents|Tab
  (params (Key :type Key%20Structure :default "None"))
  (bind _als_debug_hud (Variables|Default|GetALS_DEBUG_HUD))
  ;[1 0.4947 0.4569] DEBUG КЛАВИШИ
  (:Pressed
    (Variables|/Game/RisingSignal/Core/HUD/UI_Debug/WBP_ALS_HUD_RS.WBP_ALS_HUD_RS_C|SetShowHUD _als_debug_hud (not (Variables|/Game/RisingSignal/Core/HUD/UI_Debug/WBP_ALS_HUD_RS.WBP_ALS_HUD_RS_C|GetShowHUD _als_debug_hud)))))

(event Input|KeyboardEvents|V
  (params (Key :type Key%20Structure :default "None"))
  (bind _als_debug_hud (Variables|Default|GetALS_DEBUG_HUD))
  ;[1 0.4947 0.4569] DEBUG КЛАВИШИ
  (:Pressed
    (Variables|/Game/RisingSignal/Core/HUD/UI_Debug/WBP_ALS_HUD_RS.WBP_ALS_HUD_RS_C|SetShowCharacterInfo _als_debug_hud (not (Variables|/Game/RisingSignal/Core/HUD/UI_Debug/WBP_ALS_HUD_RS.WBP_ALS_HUD_RS_C|GetShowCharacterInfo _als_debug_hud)))))

(fn ConstructionScript)

(fn InventoryCheck
  (bind (_array_element _array_index) (Utilities|Array|ForEachLoopwithBreak (Variables|Default|GetInventoryObjects) :!label _label)
    (:LoopBody
      (if (== _array_element 0)
        (Utilities|FlowControl|Sequence
          (:then_0
            (goto _label Break))
          (:then_1
            (Variables|Default|SetEmptySlot _array_index)
            (Variables|Default|SetHasInventorySpace? true)
            (return (Variables|Default|GetHasInventorySpace?))))))
    (:Completed
      (Variables|Default|SetHasInventorySpace? false)
      (return (Variables|Default|GetHasInventorySpace?)))))

(fn PickUpItem
  (params (Item%20to%20Pickup :type Object%20Object%20Reference))
  (bind _bhasspace (CallFunction|InventoryCheck))
  (if _bhasspace
    (Utilities|Array|SetArrayElem (Variables|Default|GetInventoryObjects) (Variables|Default|GetEmptySlot) Item%20to%20Pickup)
    (bind _asbp_pick_up (Utilities|Casting|CastToBP_PickUp Item%20to%20Pickup))
    (Default|CallPickUpInventItem _asbp_pick_up (Variables|Default|GetEmptySlot))
    (else
      (Development|PrintString "Cant pickup"))))

(fn ClearInventory
  (bind _inventoryobjects (Variables|Default|GetInventoryObjects))
  (for (_ _array_index) _inventoryobjects
    (Utilities|Array|SetArrayElem _inventoryobjects _array_index 0))
  (for _array_element (Variables|/Game/RisingSignal/Core/HUD/UI_UserHUD/Widgets/WBP_Inventory.WBP_Inventory_C|GetInventoryButtons (Variables|/Game/RisingSignal/Core/HUD/UI_UserHUD/Widgets/WBP_HUD.WBP_HUD_C|GetWBP_Inventory (Variables|/Game/RisingSignal/Core/HUD/UI_UserHUD/Blueprints/BP_TestPlayerCharacter.BP_TestPlayerCharacter_C|GetHUDRef (Variables|Default|GetCharacterRef))))
    (Variables|/Game/RisingSignal/Core/HUD/UI_UserHUD/Widgets/WBP_InventorySlot.WBP_InventorySlot_C|SetForEmptyImage _array_element 0)
    (Default|SetImage _array_element)))

(fn MoveItem
  (params (From :type Integer) (To :type Integer))
  (bind _inventoryobjects (Variables|Default|GetInventoryObjects))
  (bind _inventoryobjects_2 (Variables|Default|GetInventoryObjects))
  (LocalVariables|SetLocalFrom From)
  (LocalVariables|SetLocalTo To)
  (if (Utilities|IsValid (Utilities|Array|Get(acopy) (Variables|Default|GetInventoryObjects) (LocalVariables|GetLocalTo)))
    (LocalVariables|SetLocalTempObj (Utilities|Array|Get(acopy) (Variables|Default|GetInventoryObjects) (LocalVariables|GetLocalTo)))
    (Utilities|Array|SetArrayElem _inventoryobjects_2 (LocalVariables|GetLocalTo) (Utilities|Array|Get(acopy) _inventoryobjects_2 (LocalVariables|GetLocalFrom)))
    (Utilities|Array|SetArrayElem (Variables|Default|GetInventoryObjects) (LocalVariables|GetLocalFrom) (LocalVariables|GetLocalTempObj))
    (LocalVariables|SetLocalSwapping true)
    (else
      (Utilities|Array|SetArrayElem _inventoryobjects (LocalVariables|GetLocalTo) (Utilities|Array|Get(acopy) _inventoryobjects (LocalVariables|GetLocalFrom)))
      (Utilities|Array|SetArrayElem (Variables|Default|GetInventoryObjects) (LocalVariables|GetLocalFrom) 0)
      (LocalVariables|SetLocalSwapping false)))
  (return (LocalVariables|GetLocalSwapping)))

(fn RemoveItem
  (params (InventorySlot :type Integer) (ActionSlot :type Integer) (PickupItemImage :type Texture%202D%20Object%20Reference))
  (bind _characterref (Variables|Default|GetCharacterRef))
  (bind _hudref (Variables|/Game/RisingSignal/Core/HUD/UI_UserHUD/Blueprints/BP_TestPlayerCharacter.BP_TestPlayerCharacter_C|GetHUDRef _characterref))
  (LocalVariables|SetLocalInventorySlot InventorySlot)
  (LocalVariables|SetLocalActionSlot ActionSlot)
  (LocalVariables|SetLocalImage PickupItemImage)
  (for _array_element (Variables|/Game/RisingSignal/Core/HUD/UI_UserHUD/Widgets/WBP_ActionBar.WBP_ActionBar_C|GetActionButtons (Variables|/Game/RisingSignal/Core/HUD/UI_UserHUD/Widgets/WBP_HUD.WBP_HUD_C|GetWBP_ActionBar _hudref))
    (if (== (Variables|/Game/RisingSignal/Core/HUD/UI_UserHUD/Widgets/WBP_ActionSlot.WBP_ActionSlot_C|GetForEmptyImage _array_element) (LocalVariables|GetLocalImage))
      (Variables|/Game/RisingSignal/Core/HUD/UI_UserHUD/Widgets/WBP_ActionSlot.WBP_ActionSlot_C|SetForEmptyImage _array_element 0)
      (Class|Button|SetStyle (Variables|/Game/RisingSignal/Core/HUD/UI_UserHUD/Widgets/WBP_ActionSlot.WBP_ActionSlot_C|GetButton_38 _array_element) (Variables|/Game/RisingSignal/Core/HUD/UI_UserHUD/Widgets/WBP_ActionSlot.WBP_ActionSlot_C|GetDefaultButtonStyle _array_element))))
  (Variables|/Game/RisingSignal/Core/HUD/UI_UserHUD/Widgets/WBP_InventorySlot.WBP_InventorySlot_C|SetForEmptyImage (Utilities|Array|Get(acopy) (Variables|/Game/RisingSignal/Core/HUD/UI_UserHUD/Widgets/WBP_Inventory.WBP_Inventory_C|GetInventoryButtons (Variables|/Game/RisingSignal/Core/HUD/UI_UserHUD/Widgets/WBP_HUD.WBP_HUD_C|GetWBP_Inventory _hudref)) (LocalVariables|GetLocalInventorySlot)) 0)
  (Utilities|Array|SetArrayElem (Variables|Default|GetInventoryObjects) (LocalVariables|GetLocalInventorySlot) 0))

(fn ItemWasUsed
  (params (SlotUsed :type Integer))
  (LocalVariables|SetLocalActionSlot SlotUsed)
  (LocalVariables|SetLocalImage (Variables|/Game/RisingSignal/Core/HUD/UI_UserHUD/Widgets/WBP_ActionSlot.WBP_ActionSlot_C|GetForEmptyImage (Utilities|Array|Get(acopy) (Variables|/Game/RisingSignal/Core/HUD/UI_UserHUD/Widgets/WBP_ActionBar.WBP_ActionBar_C|GetActionButtons (Variables|/Game/RisingSignal/Core/HUD/UI_UserHUD/Widgets/WBP_HUD.WBP_HUD_C|GetWBP_ActionBar (Variables|/Game/RisingSignal/Core/HUD/UI_UserHUD/Blueprints/BP_TestPlayerCharacter.BP_TestPlayerCharacter_C|GetHUDRef (Variables|Default|GetCharacterRef)))) SlotUsed))))