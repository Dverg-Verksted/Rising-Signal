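; Player interaction component that plays a montage for the type of object the character interacts with.
; InteractEvent disables character input, then switches on object type: Item (also the default) plays a pickup montage, Ladder a climb-loop montage.
; Each branch waits for the montage's sequence length before re-enabling input.
; The item branch first destroys the BP_InteractItemActor, so a failed cast leaves input disabled.
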(event Custom|InteractEvent
  (params (Mesh :type Skeletal%20Mesh%20Component%20Object%20Reference) (InteractObjectType :type String) (Character :type Actor%20Object%20Reference) (InteractActor :type Actor%20Object%20Reference))
  (Variables|Default|SetCurrentSequenceLength 0.0)
  ;[0 0 0] Отключение управления персонажем
  (Input|DisableInput Character (Game|GetPlayerController 0))
  ;[1 1 1] Выбор логики для объекта взаимодействия
  (switch string InteractObjectType
    (:Default
      ;[0 0 0] Взаимодействие с объектом ITEM(Подбираемый предмет)
      (Development|PrintString "TYPE Object: ITEM" true false "(R=0.249918,G=0.000000,B=1.000000,A=1.000000)" :!label _label)
      (bind _output_get (Variables|Default|SetAnimMontageToPlay "/ALS/ALS/RS_Animation/Interact/A_RS_PickupItem_Poses_Montage.A_RS_PickupItem_Poses_Montage"))
      (Animation|Montage|PlayMontage Mesh _output_get
        (:then
          (bind _output_get_2 (Variables|Default|SetCurrentSequenceLength (Variables|/Script/Engine.AnimSequenceBase|GetSequenceLength _output_get)))
          (Utilities|FlowControl|Delay _output_get_2)
          ;[1 1 1] Уничтожение подбираемого предмета.
          (bind _asbp_interact_item_actor (Utilities|Casting|CastToBP_InteractItemActor InteractActor))
          (Actor|DestroyActor _asbp_interact_item_actor)
          (Development|PrintString "ITEM Destroy" true false "(R=1.000000,G=0.203752,B=0.000000,A=1.000000)"))))
    (:Item
      (goto _label))
    (:Ladder
      ;[0 0 0] Взаимодействие с объектом LADDER(Лестница)
      (Development|PrintString "TYPE Object: LADDER" true false "(R=0.249918,G=0.000000,B=1.000000,A=1.000000)")
      (bind _output_get_3 (Variables|Default|SetAnimMontageToPlay "/ALS/ALS/RS_Animation/Ladder/A_RS_Ladder_Up_Loop_Montage.A_RS_Ladder_Up_Loop_Montage"))
      (Animation|Montage|PlayMontage Mesh _output_get_3
        (:then
          (bind _output_get_4 (Variables|Default|SetCurrentSequenceLength (Variables|/Script/Engine.AnimSequenceBase|GetSequenceLength _output_get_3)))
          (Utilities|FlowControl|Delay _output_get_4)))))
  ;[0 0 0] Включение управления персонажем
  (Input|EnableInput Character (Game|GetPlayerController 0)))

(event EventBeginPlay)

(event EventTick
  (params (DeltaSeconds :type Float%20%28single-precision%29)))