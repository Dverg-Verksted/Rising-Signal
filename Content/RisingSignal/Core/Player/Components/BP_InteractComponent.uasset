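; Player interaction component that plays an animation when the RisingSignal player interacts with an item actor.
; On BeginPlay it binds to the controller's OnInteract event, then disables input and picks a montage by item type: ladder climb for static items, pickup for all others.
; Input returns after a delay equal to the montage length.
; A separate PlayChangeAnimation function handles a flag-gated ladder montage, disabling input without restoring it.
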(event Custom|InteractItemEvent
  (bind _asbp_rsgame_player (Utilities|Casting|CastToBP_RSGamePlayer (Components|GetOwner)))
  (Variables|Default|SetPlayer _asbp_rsgame_player)
  (bind _asbp_interact_item_actor (Utilities|Casting|CastToBP_InteractItemActor (Class|InteractComponent|GetInteractItem)))
  (Variables|Default|SetInteractItem _asbp_interact_item_actor)
  (Variables|Default|SetCurrentSequenceLength 0.0)
  ;[0 0 0] Отключение управления персонажем
  (Input|DisableInput (Variables|Default|GetPlayer) (Game|GetPlayerController 0))
  ;[1 1 1] Выбор логики для объекта взаимодействия
  (switch Utilities|FlowControl|Switch|SwitchonETypeItem (Utilities|Struct|BreakDataInteract (Class|InteractItemActor|GetItemData (Variables|Default|GetInteractItem)))
    (:StaticItem
      ;[0 0 0] Взаимодействие с объектом LADDER(Лестница)
      (Development|PrintString "TYPE Object: LADDER" true false "(R=0.152017,G=0.000000,B=1.000000,A=1.000000)")
      (bind _output_get (Variables|Default|SetAnimMontageToPlay "/ALS/ALS/RS_Animation/Ladder/A_RS_Ladder_Up_Loop_Montage.A_RS_Ladder_Up_Loop_Montage"))
      (Animation|Montage|PlayMontage (Variables|/Script/Engine.Character|GetMesh (Variables|Default|GetPlayer)) _output_get
        (:then
          (bind _output_get_2 (Variables|Default|SetCurrentSequenceLength (Variables|/Script/Engine.AnimSequenceBase|GetSequenceLength _output_get)))
          (Utilities|FlowControl|Delay _output_get_2))))
    (:InvItem
      ;[0 0 0] Взаимодействие с объектом ITEM(Подбираемый предмет)
      (Development|PrintString "TYPE Object: ITEM" true false "(R=0.094178,G=0.000000,B=1.000000,A=1.000000)" :!label _label)
      (bind _output_get_3 (Variables|Default|SetAnimMontageToPlay "/ALS/ALS/RS_Animation/Interact/A_RS_PickupItem_Poses_Montage.A_RS_PickupItem_Poses_Montage"))
      (Animation|Montage|PlayMontage (Variables|/Script/Engine.Character|GetMesh (Variables|Default|GetPlayer)) _output_get_3
        (:then
          (bind _output_get_4 (Variables|Default|SetCurrentSequenceLength (Variables|/Script/Engine.AnimSequenceBase|GetSequenceLength _output_get_3)))
          (Utilities|FlowControl|Delay _output_get_4))))
    (:NoteItem
      (goto _label))
    (:AudioItem
      (goto _label))
    (:PhotoItem
      (goto _label)))
  ;[0 0 0] Включение управления персонажем
  (Input|EnableInput (Variables|Default|GetPlayer) (Game|GetPlayerController 0)))

(event EventBeginPlay
  (bind _asbp_rsgame_player (Utilities|Casting|CastToBP_RSGamePlayer (Components|GetOwner)))
  (bind _asrsgame_player_controller (Utilities|Casting|CastToRSGamePlayerController (Pawn|GetController _asbp_rsgame_player)))
  (EventDispatchers|BindEventtoOnInteract _asrsgame_player_controller (delegate Custom|InteractItemEvent)))

(event EventTick
  (params (DeltaSeconds :type Float%20%28single-precision%29)))