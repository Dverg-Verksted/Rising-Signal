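; Portal actor that teleports Characters entering its mesh to a linked destination teleporter.
; The destination preserves the Character's offset from the source portal and, unless rotation is maintained, aligns actor and control rotation to itself.
; Arrivals are tracked until they leave the portal mesh, preventing an immediate bounce back.
; The construction script rejects self-links and tints a dynamic material with the portal color, or grey when unlinked.
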(event OnComponentBeginOverlap(PortalMesh)
  (params (OverlappedComponent :type Primitive%20Component%20Object%20Reference) (OtherActor :type Actor%20Object%20Reference) (OtherComp :type Primitive%20Component%20Object%20Reference) (OtherBodyIndex :type Integer) (bFromSweep :type Boolean) (SweepResult :type Hit%20Result%20Structure%20%28by%20ref%29))
  (if (CallFunction|CanActorTeleport? OtherActor)
    (bind _destinationteleporter (Variables|Default|GetDestinationTeleporter)
      (:then
        (CallFunction|IncomingTeleport _destinationteleporter OtherActor self))
      (:else))))

(event OnComponentEndOverlap(PortalMesh)
  (params (OverlappedComponent :type Primitive%20Component%20Object%20Reference) (OtherActor :type Actor%20Object%20Reference) (OtherComp :type Primitive%20Component%20Object%20Reference) (OtherBodyIndex :type Integer))
  (Utilities|Array|RemoveItem (Variables|Default|GetIncomingActors) OtherActor))

(event Custom|IncomingTeleport
  (params (Incoming%20Actor :type Actor%20Object%20Reference) (Invoking%20Teleporter :type BP%20Teleport%20Instace%20Object%20Reference))
  (CallFunction|HandleIncommingTeleport Incoming%20Actor Invoking%20Teleporter))

(fn ConstructionScript
  (if (== (Variables|Default|GetDestinationTeleporter) self)
    (Variables|Default|SetDestinationTeleporter 0))
  (bind _returnvalue (Rendering|Material|CreateDynamicMaterialInstance "/Game/RisingSignal/Core/Teleport/M_TeleportMaterial.M_TeleportMaterial" "None" "None" :!class /Script/Engine.KismetMaterialLibrary))
  (bind _output_get (LocalVariables|SetMaterialInstance _returnvalue))
  (Rendering|Material|SetMaterial (Variables|Default|GetPortalMesh) 0 _output_get)
  (Rendering|Material|SetVectorParameterValue (LocalVariables|GetMaterialInstance) "Color" (select (Utilities|IsValid (Variables|Default|GetDestinationTeleporter)) (Variables|Default|GetColor) "(R=0.500000,G=0.500000,B=0.500000,A=1.000000)") :!class /Script/Engine.MaterialInstanceDynamic))

(fn CanActorTeleport?
  (params (Actor :type Actor%20Object%20Reference))
  (Utilities|Casting|CastToCharacter Actor
    (:then
      (return (not (Utilities|Array|ContainsItem (Variables|Default|GetIncomingActors) Actor))))
    (:CastFailed
      (return false))))

(fn HandleIncommingTeleport
  (params (Incoming%20Actor :type Actor%20Object%20Reference) (Invocking%20Teleporter :type BP%20Teleport%20Instace%20Object%20Reference))
  (bind _returnvalue (Transformation|GetActorRotation))
  (bind _returnvalue_2 (Game|GetInstigatorController Incoming%20Actor))
  (if (not (Utilities|Array|ContainsItem (Variables|Default|GetIncomingActors) Incoming%20Actor))
    (Utilities|Array|Add (Variables|Default|GetIncomingActors) Incoming%20Actor)
    (Transformation|SetActorLocation Incoming%20Actor (+ (Transformation|GetActorLocation Incoming%20Actor) (- (Transformation|GetActorLocation) (Transformation|GetActorLocation Invocking%20Teleporter))) false true)
    (if (not (Variables|Default|GetMaintaingActorRotation))
      (Transformation|SetActorRotation Incoming%20Actor _returnvalue)
      (Utilities|IsValid _returnvalue_2
        (:Is%20Valid
          (Pawn|SetControlRotation _returnvalue_2 _returnvalue))))))