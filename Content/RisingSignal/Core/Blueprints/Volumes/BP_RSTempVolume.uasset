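; BP_RSTempVolume is a volume that alters how an ability state changes for actors inside it.
; On begin overlap, it passes its AbilityType and ChangedValueModifier to the actor's RSAbilitySystem component through SetChangeValue.
; On end overlap, it sends the reciprocal of the modifier, which suggests a multiplicative effect undone on exit.
; Actors without that component are ignored.
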(event Collision|EventActorBeginOverlap
  (params (OtherActor :type Actor%20Object%20Reference))
  (bind _returnvalue (Actor|GetComponentbyClass OtherActor "/Script/RisingSignal.RSAbilitySystem"))
  (Utilities|IsValid _returnvalue
    (:Is%20Valid
      (Class|RSAbilitySystem|SetChangeValue _returnvalue (Variables|Default|GetAbilityType) (Variables|Default|GetChangedValueModifier)))))

(event Collision|EventActorEndOverlap
  (params (OtherActor :type Actor%20Object%20Reference))
  (bind _returnvalue (Actor|GetComponentbyClass OtherActor "/Script/RisingSignal.RSAbilitySystem"))
  (Utilities|IsValid _returnvalue
    (:Is%20Valid
      (Class|RSAbilitySystem|SetChangeValue _returnvalue (Variables|Default|GetAbilityType) (/ 1.0 (Variables|Default|GetChangedValueModifier))))))

(fn ConstructionScript)