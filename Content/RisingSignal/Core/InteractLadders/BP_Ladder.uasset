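; Ladder segment actor that moves BP_RSGamePlayer in and out of the ALS ladder state through trigger boxes.
; The start box turns the player to the Arrow and sets ladder mode; leaving it restores walking only on OutPoint segments, which end a composite ladder.
; For top entry, side triggers arm or disarm the UpIn box, which disables input, snaps the player to arrow markers and optionally plays a descent montage.
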(event OnComponentBeginOverlap(BoxCollisionStart)
  (params (OverlappedComponent :type Primitive%20Component%20Object%20Reference) (OtherActor :type Actor%20Object%20Reference) (OtherComp :type Primitive%20Component%20Object%20Reference) (OtherBodyIndex :type Integer) (bFromSweep :type Boolean) (SweepResult :type Hit%20Result%20Structure%20%28by%20ref%29))
  (bind _asbp_rsgame_player (Utilities|Casting|CastToBP_RSGamePlayer OtherActor))
  (Variables|/Game/RisingSignal/Core/Player/BP_RSGamePlayer.BP_RSGamePlayer_C|SetIsOnLadder _asbp_rsgame_player true)
  (Variables|Default|SetBPRSGamePlayerRef _asbp_rsgame_player)
  ;[0 0 0] Установка режима поведения карабканье по лестнице
  (Class|AlsCharacter|SetOverlayMode _asbp_rsgame_player "(TagName=\"Als.LocomotionMode.InLadder\")")
  ;[0 0 0] Поворот персонажа в положение Arrow
  (bind _time (Timeline|TL_RotationTime PlayFromStart)
    (:Update
      (Transformation|SetActorRotation (Variables|Default|GetBPRSGamePlayerRef) (Math|Rotator|Lerp(Rotator) (Transformation|GetActorRotation (Variables|Default|GetBPRSGamePlayerRef)) (Transformation|GetWorldRotation (Variables|Default|GetArrow)) _time) true)
      (Input|EnableInput (Variables|Default|GetBPRSGamePlayerRef) (Game|GetPlayerController 0)))))

(event OnComponentEndOverlap(BoxCollisionStart)
  (params (OverlappedComponent :type Primitive%20Component%20Object%20Reference) (OtherActor :type Actor%20Object%20Reference) (OtherComp :type Primitive%20Component%20Object%20Reference) (OtherBodyIndex :type Integer))
  ;[0 0 0] Является ли участок лестницы последним элементом в цепочке составной лестницы
  (if (Variables|Default|GetOutPoint)
    (bind _asbp_rsgame_player (Utilities|Casting|CastToBP_RSGamePlayer OtherActor))
    (Variables|/Game/RisingSignal/Core/Player/BP_RSGamePlayer.BP_RSGamePlayer_C|SetIsOnLadder _asbp_rsgame_player false)
    (Pawn|Components|CharacterMovement|SetMovementMode (Variables|/Script/ALS.AlsCharacter|GetAlsCharacterMovement _asbp_rsgame_player) "MOVE_Walking" 0)
    ;[0 0 0] Установка режима поведения по умолчанию
    (Class|AlsCharacter|SetOverlayMode _asbp_rsgame_player "(TagName=\"Als.OverlayMode.Default\")")
    (Collision|SetCollisionEnabled (Variables|Default|GetBoxCollisionStart) "NoCollision")
    (Utilities|FlowControl|Delay 1.2)
    (Collision|SetCollisionEnabled (Variables|Default|GetBoxCollisionStart) "QueryOnly")
    (else
      (Collision|SetCollisionEnabled (Variables|Default|GetBoxCollisionStart) "QueryOnly"))))

(event OnComponentBeginOverlap(SM_LadderMiddle)
  (params (OverlappedComponent :type Primitive%20Component%20Object%20Reference) (OtherActor :type Actor%20Object%20Reference) (OtherComp :type Primitive%20Component%20Object%20Reference) (OtherBodyIndex :type Integer) (bFromSweep :type Boolean) (SweepResult :type Hit%20Result%20Structure%20%28by%20ref%29)))

(event OnComponentBeginOverlap(BoxCollisionUpIn)
  (params (OverlappedComponent :type Primitive%20Component%20Object%20Reference) (OtherActor :type Actor%20Object%20Reference) (OtherComp :type Primitive%20Component%20Object%20Reference) (OtherBodyIndex :type Integer) (bFromSweep :type Boolean) (SweepResult :type Hit%20Result%20Structure%20%28by%20ref%29))
  (bind _asbp_rsgame_player (Utilities|Casting|CastToBP_RSGamePlayer OtherActor))
  (bind _output_get (Variables|Default|SetBPRSGamePlayerRef _asbp_rsgame_player))
  (Input|DisableInput _output_get (Game|GetPlayerController 0))
  (Collision|SetCollisionEnabled (Variables|Default|GetBoxCollisionUpIn) "NoCollision")
  ;[0 0 0] Поворот персонажа в положение Arrow
  (bind _time (Timeline|TL_Rotate PlayFromStart)
    (:Update
      (Utilities|FlowControl|Sequence
        (:then_0
          (Transformation|SetActorRotation (Variables|Default|GetBPRSGamePlayerRef) (Transformation|GetWorldRotation (Variables|Default|GetArrowUpInPosition)) true)
          (Variables|/Game/RisingSignal/Core/Player/BP_RSGamePlayer.BP_RSGamePlayer_C|SetMoveForwardIntValue _asbp_rsgame_player 1)
          ;[1 1 1] Включение анимации подготовки к спуску по лестнице (Alpha)
          (if (Variables|Default|GetUpInAnimation)
            (bind _output_get_2 (Variables|Default|SetAnimMontageToPlay "/ALS/ALS/RS_Animation/Ladder/A_RS_Ladder_Up_In_Montage.A_RS_Ladder_Up_In_Montage"))
            (Animation|Montage|PlayMontage (Variables|/Script/Engine.Character|GetMesh _asbp_rsgame_player) _output_get_2
              (:then
                (Utilities|FlowControl|Delay (Variables|/Script/Engine.AnimSequenceBase|GetSequenceLength _output_get_2)))
              (:OnCompleted
                _))
            (else
              (Utilities|FlowControl|Delay 0.3)))
          ;[0 0 0] Перемещение персонажа в положение Arrow
          (Transformation|SetActorLocation (Variables|Default|GetBPRSGamePlayerRef) (Transformation|GetWorldLocation (Variables|Default|GetArrowUpInPosition)) false true)
          (Class|AlsCharacter|SetOverlayMode (Variables|Default|GetBPRSGamePlayerRef) "(TagName=\"Als.LocomotionMode.InLadder\")"))
        (:then_1
          ;[0 0 0] Перемещение персонажа в положение Arrow
          (Transformation|SetActorLocation (Variables|Default|GetBPRSGamePlayerRef) (Transformation|GetWorldLocation (Variables|Default|GetArrowUpInStartPosition)) false true))))))

(event OnComponentBeginOverlap(BoxCollisionUpIn_Enabled)
  (params (OverlappedComponent :type Primitive%20Component%20Object%20Reference) (OtherActor :type Actor%20Object%20Reference) (OtherComp :type Primitive%20Component%20Object%20Reference) (OtherBodyIndex :type Integer) (bFromSweep :type Boolean) (SweepResult :type Hit%20Result%20Structure%20%28by%20ref%29))
  (bind _asbp_rsgame_player (Utilities|Casting|CastToBP_RSGamePlayer OtherActor))
  (Variables|Default|SetBPRSGamePlayerRef _asbp_rsgame_player)
  ;[0 0 0] Включение колизии для проигрывания анимации подготовки к спуску по лестнице
  (Collision|SetCollisionEnabled (Variables|Default|GetBoxCollisionUpIn) "QueryOnly"))

(event OnComponentBeginOverlap(BoxCollisionUpIn_Disabled)
  (params (OverlappedComponent :type Primitive%20Component%20Object%20Reference) (OtherActor :type Actor%20Object%20Reference) (OtherComp :type Primitive%20Component%20Object%20Reference) (OtherBodyIndex :type Integer) (bFromSweep :type Boolean) (SweepResult :type Hit%20Result%20Structure%20%28by%20ref%29))
  (bind _asbp_rsgame_player (Utilities|Casting|CastToBP_RSGamePlayer OtherActor))
  (Variables|Default|SetBPRSGamePlayerRef _asbp_rsgame_player)
  ;[0 0 0] Включение колизии для проигрывания анимации подготовки к спуску по лестнице
  (Collision|SetCollisionEnabled (Variables|Default|GetBoxCollisionUpIn) "NoCollision"))

(event OnComponentEndOverlap(BoxCollisionUpIn)
  (params (OverlappedComponent :type Primitive%20Component%20Object%20Reference) (OtherActor :type Actor%20Object%20Reference) (OtherComp :type Primitive%20Component%20Object%20Reference) (OtherBodyIndex :type Integer))
  (bind _asbp_rsgame_player (Utilities|Casting|CastToBP_RSGamePlayer OtherActor))
  (if (not (Variables|/Game/RisingSignal/Core/Player/BP_RSGamePlayer.BP_RSGamePlayer_C|GetIsOnLadder _asbp_rsgame_player))
    (Pawn|Components|CharacterMovement|SetMovementMode (Variables|/Script/ALS.AlsCharacter|GetAlsCharacterMovement _asbp_rsgame_player) "MOVE_Walking" 0)
    ;[0 0 0] Установка режима поведения по умолчанию
    (Class|AlsCharacter|SetOverlayMode _asbp_rsgame_player "(TagName=\"Als.OverlayMode.Default\")")))

(event EventBeginPlay
  ;[0 0 0] Установка видимости вспомогательных элементов BP_Ladder
  (if (Variables|Default|GetSupportiveMeshVisible)
    (Rendering|SetVisibility (Variables|Default|GetSM_LadderMiddle) true false)
    (else
      (Rendering|SetVisibility (Variables|Default|GetSM_LadderDown) false false))))

(event Collision|EventActorBeginOverlap
  (params (OtherActor :type Actor%20Object%20Reference)))

(event EventTick
  (params (DeltaSeconds :type Float%20%28single-precision%29)))

(fn ConstructionScript)