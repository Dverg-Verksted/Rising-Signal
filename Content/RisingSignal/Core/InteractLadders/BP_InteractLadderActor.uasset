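; Ladder interactable actor that carries the player up a spline when they overlap its entry collision.
; On overlap it disables the exit collision, switches the player's ALS overlay mode to InLadder, and starts a timeline that teleports them along SplineUp.
; When the timeline finishes, it restores the default overlay and runs a delayed DoOnce reset.
; Only upward movement is implemented, and the node re-enabling exit collision is unconnected.
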(event OnComponentBeginOverlap(CollisionIn)
  (params (OverlappedComponent :type Primitive%20Component%20Object%20Reference) (OtherActor :type Actor%20Object%20Reference) (OtherComp :type Primitive%20Component%20Object%20Reference) (OtherBodyIndex :type Integer) (bFromSweep :type Boolean) (SweepResult :type Hit%20Result%20Structure%20%28by%20ref%29))
  (bind _asbp_rsgame_player (Utilities|Casting|CastToBP_RSGamePlayer OtherActor))
  (Collision|SetCollisionEnabled (Variables|Default|GetCollisionOut) "NoCollision")
  (Class|AlsCharacter|SetOverlayMode _asbp_rsgame_player "(TagName=\"Als.LocomotionMode.InLadder\")")
  (Utilities|FlowControl|Sequence
    (:then_0
      (bind _movingtime (Timeline|TL_MovingStateUp Play)
        (:Update
          (bind _output_get (Variables|Default|SetCurrentMovingScale _movingtime))
          (Transformation|SetWorldLocation (Variables|/Script/Engine.Actor|GetRootComponent _asbp_rsgame_player) (Spline|GetLocationatTime (Variables|Default|GetSplineUp) _output_get "World" false) false false))
        (:Finished
          (Class|AlsCharacter|SetOverlayMode _asbp_rsgame_player "(TagName=\"Als.OverlayMode.Default\")")
          (Utilities|FlowControl|Delay 1.2)
          (goto _label Reset))))
    (:then_1
      (Utilities|FlowControl|DoOnce false :!label _label
        (:Completed
          (Timeline|TL_MovingStateUp SetNewTime))))))

(event EventBeginPlay
  (|CallParentFunction)
  ;[0 0 0] Установка типа объекта "Лестница"
  (Variables|Default|SetObjectType "Ladder"))

(event EventTick
  (params (DeltaSeconds :type Float%20%28single-precision%29))
  (|CallParentFunction DeltaSeconds) ; This node is disabled and will not be called.\nDrag off pins to build functionality.
)

(fn ConstructionScript
  (|CallParentFunction))