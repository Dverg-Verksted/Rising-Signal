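; BP_Rope is a grabbable rope actor that swings when grabbed.
; Capsule overlap sends OnGrabRopeMessage with the rope to the overlapping actor, unfiltered, then calls AddSwingingForce with the grip force.
; That event pushes CableEnd with a mass-independent force, its sign set by InertionLR.
; Swing is capped by applying force only while CableEnd hangs more than SwingLimit below the actor origin.
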(event OnComponentBeginOverlap(Capsule)
  (params (OverlappedComponent :type Primitive%20Component%20Object%20Reference) (OtherActor :type Actor%20Object%20Reference) (OtherComp :type Primitive%20Component%20Object%20Reference) (OtherBodyIndex :type Integer) (bFromSweep :type Boolean) (SweepResult :type Hit%20Result%20Structure%20%28by%20ref%29))
  ;[1 1 1] Захват верёвки
  (Class|BPIPlayer|OnGrabRope(Message) OtherActor self)
  ;[1 1 1] Добавление инерции при захвате верёвки
  (CallFunction|AddSwingingForce (Variables|Default|GetSwingForceWhenGrip)))

(event Custom|AddSwingingForce
  (params (SwingForce :type Vector))
  ;[1 1 1] Добавление силы для раскачивания верёвки
  (if (> (- (.z (Transformation|GetActorLocation)) (.z (Transformation|GetWorldLocation (Variables|Default|GetCableEnd)))) (Variables|Default|GetSwingLimit))
    (if (Variables|Default|GetInertionLR)
      ;[1 1 1] Раскачивание верёвки слева направо при захвате
      (Physics|AddForce (Variables|Default|GetCableEnd) (* SwingForce 2.5e+02) "None" true)
      (else
        ;[1 1 1] Раскачивание верёвки справа налево при захвате
        (Physics|AddForce (Variables|Default|GetCableEnd) (* (* SwingForce -1.0) 2.5e+02) "None" true)))))

(event EventBeginPlay)

(event Collision|EventActorBeginOverlap
  (params (OtherActor :type Actor%20Object%20Reference)))

(event EventTick
  (params (DeltaSeconds :type Float%20%28single-precision%29)))

(fn ConstructionScript)