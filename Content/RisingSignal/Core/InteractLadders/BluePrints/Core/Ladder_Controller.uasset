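; Player character component that mediates between the Character and interactable objects such as ladders.
; Input events drive movement, camera and jump, with an optional custom-input mode that forwards axes to the current object through BPI_ObjectControls.
; Jump and action pick the overlapped object best aligned by angle, falling back to a box overlap search.
; Interface calls let objects adjust movement, capsule and montages, or ease the player to a floor-adjusted target transform on Tick.
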(event Custom|MoveForwardInput
  (params (Axis :type Float%20%28single-precision%29))
  (bind _currentobjectactorptr (Variables|Default|GetCurrentObjectActorPtr))
  (bind _usecustominput (Variables|Default|GetUseCustomInput))
  ;[1 1 1] Main input
  ;;[1 1 1] Forward
  (if (Variables|Default|GetInputEnable)
    (Variables|Default|SetForwardAxisValue Axis)
    (Pawn|Input|AddMovementInput (Variables|Default|GetPlayerCharacter) (Math|Vector|SelectVector (Variables|Default|GetCustomForwardVector) (Math|Vector|GetForwardVector (Math|Rotator|MakeRotator 0.0 0.0 (.yaw (Pawn|GetControlRotation (Variables|Default|GetPlayerCharacter) :!class /Script/Engine.Pawn)))) _usecustominput) (Math|Float|SelectFloat (Variables|Default|GetCustomForwardAxis) (Variables|Default|GetForwardAxisValue) _usecustominput) false)
    (if _usecustominput
      (if (and (Utilities|DoesObjectImplementInterface _currentobjectactorptr "/Game/RisingSignal/Core/InteractLadders/BluePrints/Core/BPI_ObjectControls.BPI_ObjectControls_C") (Utilities|Enum|NotEqual(Enum) (Variables|Default|GetCurrentObjectType) "NewEnumerator1"))
        (Class|BPIObjectControls|MoveForwardBPI(Message) _currentobjectactorptr (Variables|Default|GetForwardAxisValue) (Variables|Default|GetPlayerCharacter))))
    (else
      (Variables|Default|SetForwardAxisValue 0.0))))

(event Custom|MoveRightInput
  (params (Axis :type Float%20%28single-precision%29))
  (bind _currentobjectactorptr (Variables|Default|GetCurrentObjectActorPtr))
  (bind _usecustominput (Variables|Default|GetUseCustomInput))
  ;[1 1 1] Main input
  ;;[1 1 1] Right
  (if (Variables|Default|GetInputEnable)
    (Variables|Default|SetRightAxisValue Axis)
    (Pawn|Input|AddMovementInput (Variables|Default|GetPlayerCharacter) (Math|Vector|SelectVector (Variables|Default|GetCustomRightVector) (Math|Vector|GetRightVector (Math|Rotator|MakeRotator 0.0 0.0 (.yaw (Pawn|GetControlRotation (Variables|Default|GetPlayerCharacter) :!class /Script/Engine.Pawn)))) _usecustominput) (Math|Float|SelectFloat (Variables|Default|GetCustomRightAxis) (Variables|Default|GetRightAxisValue) _usecustominput) false)
    (if _usecustominput
      (if (and (Utilities|DoesObjectImplementInterface _currentobjectactorptr "/Game/RisingSignal/Core/InteractLadders/BluePrints/Core/BPI_ObjectControls.BPI_ObjectControls_C") (Utilities|Enum|NotEqual(Enum) (Variables|Default|GetCurrentObjectType) "NewEnumerator1"))
        (Class|BPIObjectControls|MoveRightBPI(Message) _currentobjectactorptr (Variables|Default|GetRightAxisValue) (Variables|Default|GetPlayerCharacter))))
    (else
      (Variables|Default|SetRightAxisValue 0.0))))

(event Custom|AddYawInput
  (params (Val :type Float%20%28single-precision%29))
  ;[1 1 1] Additional Input handles
  ;;[1 1 1] Yaw
  (if (Variables|Default|GetCameraEnable)
    (Pawn|Input|AddControllerYawInput (Variables|Default|GetPlayerCharacter) Val)))

(event Custom|AddPitchInput
  (params (Val :type Float%20%28single-precision%29))
  ;[1 1 1] Additional Input handles
  ;;[1 1 1] Pitch
  (if (Variables|Default|GetCameraEnable)
    (Pawn|Input|AddControllerPitchInput (Variables|Default|GetPlayerCharacter) Val)))

(event Custom|TryToFindOverlappedObjects
  (bind _character_capsule (Variables|Default|GetCharacter_Capsule))
  (bind _overlapextent (Variables|APCController|GetOverlapExtent))
  ;[1 1 1] Overlapped object find function. Try to find any gameplay object within specified volume ahead the character
  (bind _capsuleradius (CallFunction|GetCapsuleRadiusBPI))
  (bind _outactors (Collision|BoxOverlapActors (+ (* (Math|Vector|GetForwardVector _character_capsule) (+ _capsuleradius (Variables|APCController|GetOverlapExtent))) (Transformation|GetWorldLocation _character_capsule)) (Math|Vector|MakeVector _overlapextent _overlapextent 7e+01) (Utilities|Array|MakeArray "ObjectTypeQuery2") "/Script/Engine.Actor" (Utilities|Array|MakeArray (Variables|Default|GetPlayerCharacter)) :!class /Script/Engine.KismetSystemLibrary))
  (if (> (Utilities|Array|Length _outactors) 0)
    (for _array_element _outactors
      (if (Utilities|DoesObjectImplementInterface _array_element "/Game/RisingSignal/Core/InteractLadders/BluePrints/Core/BPI_ObjectControls.BPI_ObjectControls_C")
        (Class|BPIObjectControls|UpdateOverlapsBPI(Message) _array_element)))))

(event Custom|UpdatePlayerRotation
  ;[1 1 1] Update Player rotation
  (Variables|Default|SetPlayerRotation (Transformation|GetActorRotation (Variables|Default|GetPlayerCharacter))))

(event Custom|FinishActorTransition
  (bind _currentobjectactorptr (Variables|Default|GetCurrentObjectActorPtr))
  ;[1 1 1] Transition of player actor to destination location
  (Utilities|IsValid _currentobjectactorptr
    (:Is%20Valid
      (Class|BPIObjectControls|TransitionCompleteBPI(Message) _currentobjectactorptr (Variables|Default|GetPlayerCharacter)))
    (:Is%20Not%20Valid
      _))
  (Variables|Default|SetInputEnable true))

(event Custom|ActionOneInput
  (bind _playercharacter (Variables|Default|GetPlayerCharacter))
  ;[1 1 1] JUMP, Action 1 events
  (if (not (Variables|Default|GetAimMode))
    (Variables|Default|SetAction1Pressed true)
    (if (> (Utilities|Array|Length (Variables|Default|GetOverlappedObjects)) 0)
      _
      (else
        (CallFunction|TrytoFindOverlappedObjects)))
    (bind (_actor _type) (CallFunction|GetOverlappedObject))
    (if (Utilities|Enum|NotEqual(Enum) _type "NewEnumerator1")
      (Variables|Default|SetCurrentObjectActorPtr _actor)
      (Variables|Default|SetCurrentObjectType _type)
      (if (Variables|Default|GetAction1Pressed)
        (Class|BPIObjectControls|ActionOneBPI(Message) (Variables|Default|GetCurrentObjectActorPtr) _playercharacter)
        (Variables|Default|SetAction1Pressed false :!label _label)
        (Variables|Default|SetJumpPressed false)
        (else
          (if (Variables|Default|GetJumpPressed) :!label _label_2
            (if (Utilities|Enum|Equal(Enum) (Variables|Default|GetCurrentObjectType) "NewEnumerator3")
              (goto _label)
              (else
                (Character|Jump _playercharacter)
                (goto _label))))))
      (else
        (Variables|Default|SetCurrentObjectActorPtr 0)
        (Variables|Default|SetCurrentObjectType "NewEnumerator1")
        (goto _label_2)))))

(event Custom|JumpInput
  (bind _playercharacter (Variables|Default|GetPlayerCharacter))
  ;[1 1 1] JUMP, Action 1 events
  (if (Variables|Default|GetIsJumpEnabled)
    (if (not (Variables|Default|GetAimMode))
      (Variables|Default|SetJumpPressed true)
      (if (> (Utilities|Array|Length (Variables|Default|GetOverlappedObjects)) 0)
        _
        (else
          (CallFunction|TrytoFindOverlappedObjects)))
      (bind (_actor _type) (CallFunction|GetOverlappedObject))
      (if (Utilities|Enum|NotEqual(Enum) _type "NewEnumerator1")
        (Variables|Default|SetCurrentObjectActorPtr _actor)
        (Variables|Default|SetCurrentObjectType _type)
        (if (Variables|Default|GetAction1Pressed)
          (Class|BPIObjectControls|ActionOneBPI(Message) (Variables|Default|GetCurrentObjectActorPtr) _playercharacter)
          (Variables|Default|SetAction1Pressed false :!label _label)
          (Variables|Default|SetJumpPressed false)
          (else
            (if (Variables|Default|GetJumpPressed) :!label _label_2
              (if (Utilities|Enum|Equal(Enum) (Variables|Default|GetCurrentObjectType) "NewEnumerator3")
                (goto _label)
                (else
                  (Character|Jump _playercharacter)
                  (goto _label))))))
        (else
          (Variables|Default|SetCurrentObjectActorPtr 0)
          (Variables|Default|SetCurrentObjectType "NewEnumerator1")
          (goto _label_2))))))

(event Custom|MoveUpInput
  (params (Axis :type Float%20%28single-precision%29))
  (bind _currentobjectactorptr (Variables|Default|GetCurrentObjectActorPtr))
  ;[1 1 1] Additional Input handles
  ;;[1 1 1] Up
  (if (Variables|Default|GetInputEnable)
    (Variables|Default|SetUpAxisValue Axis)
    (if (Variables|Default|GetUseCustomInput)
      (if (and (Utilities|DoesObjectImplementInterface _currentobjectactorptr "/Game/RisingSignal/Core/InteractLadders/BluePrints/Core/BPI_ObjectControls.BPI_ObjectControls_C") (Utilities|Enum|NotEqual(Enum) (Variables|Default|GetCurrentObjectType) "NewEnumerator1"))
        (Class|BPIObjectControls|MoveUpBPI(Message) _currentobjectactorptr (Variables|Default|GetUpAxisValue) (Variables|Default|GetPlayerCharacter))))
    (else
      (Variables|Default|SetUpAxisValue 0.0))))

(event Custom|MoveDownInput
  (params (Axis :type Float%20%28single-precision%29))
  (bind _currentobjectactorptr (Variables|Default|GetCurrentObjectActorPtr))
  ;[1 1 1] Additional Input handles
  ;;[1 1 1] Down
  (if (Variables|Default|GetInputEnable)
    (Variables|Default|SetUpAxisValue Axis)
    (if (Variables|Default|GetUseCustomInput)
      (if (and (Utilities|DoesObjectImplementInterface _currentobjectactorptr "/Game/RisingSignal/Core/InteractLadders/BluePrints/Core/BPI_ObjectControls.BPI_ObjectControls_C") (Utilities|Enum|NotEqual(Enum) (Variables|Default|GetCurrentObjectType) "NewEnumerator1"))
        (Class|BPIObjectControls|MoveUpBPI(Message) _currentobjectactorptr (Variables|Default|GetUpAxisValue) (Variables|Default|GetPlayerCharacter))))
    (else
      (Variables|Default|SetUpAxisValue 0.0))))

(event EventBeginPlay
  (bind _playertag (CallFunction|LIBGetPlayerTag))
  ;[0.1297 1 0.3051] Initialization
  (bind _ascharacter (Utilities|Casting|CastToCharacter (Components|GetOwner)))
  (Utilities|Array|Add (Variables|/Script/Engine.Actor|GetTags _ascharacter) _playertag)
  (Variables|Default|SetOwnerTag _playertag)
  (bind _output_get (Variables|Default|SetPlayerCharacter _ascharacter))
  (bind _output_get_2 (Variables|Default|SetCharacter_Capsule (Variables|/Script/Engine.Character|GetCapsuleComponent _output_get)))
  (Variables|Default|SetInitCapsuleRadius (Variables|/Script/Engine.CapsuleComponent|GetCapsuleRadius _output_get_2))
  (bind _output_get_3 (Variables|Default|SetCharacter_MovementComp (Variables|/Script/Engine.Character|GetCharacterMovement _output_get)))
  (Variables|/Script/Engine.CharacterMovementComponent|SetbOrientRotationToMovement _output_get_3 true)
  ;;[1 1 1] Try to find SpringArm component
  (bind _springarmcomp (CallFunction|TrytoFindSpringArm))
  (bind _output_get_4 (Variables|Default|SetCharacter_CameraBoom _springarmcomp))
  (Utilities|IsValid _output_get_4
    (:Is%20Valid
      (Variables|Default|SetInitSpringArmLenght (Variables|/Script/Engine.SpringArmComponent|GetTargetArmLength (Variables|Default|GetCharacter_CameraBoom)))
      (Variables|Default|SetInitSocketOffset (Variables|/Script/Engine.SpringArmComponent|GetSocketOffset (Variables|Default|GetCharacter_CameraBoom))))
    (:Is%20Not%20Valid
      (CallFunction|LIBDebugPrint "APC_Controller: Can't find SpringArm component" "(R=1.000000,G=0.000000,B=0.000000,A=1.000000)" 4.0)))
  ;;[1 1 1] Try to find Main Camera component
  (bind _cameracomp (CallFunction|TrytoFindCamera))
  (bind _output_get_5 (Variables|Default|SetCharacter_Camera _cameracomp))
  (Utilities|IsValid _output_get_5
    (:Is%20Valid
      (Variables|Default|SetInitCameraFOV (Variables|/Script/Engine.CameraComponent|GetFieldOfView (Variables|Default|GetCharacter_Camera))))
    (:Is%20Not%20Valid
      (CallFunction|LIBDebugPrint "APC_Controller: Can't find Camera component" "(R=1.000000,G=0.000000,B=0.000000,A=1.000000)" 4.0)))
  (Variables|Default|SetCharacter_SkeletalMesh (Variables|/Script/Engine.Character|GetMesh (Variables|Default|GetPlayerCharacter)))
  (Variables|Default|SetCharacter_AnimInstance (Components|SkeletalMesh|GetAnimInstance (Variables|/Script/Engine.Character|GetMesh (Variables|Default|GetPlayerCharacter))))
  (Variables|Default|SetDefaultWalkSpeed (Variables|/Script/Engine.CharacterMovementComponent|GetMaxWalkSpeed (Variables|Default|GetCharacter_MovementComp)))
  (Variables|Default|SetCurrentObjectActorPtr 0)
  (Variables|Default|SetCurrentObjectType "NewEnumerator1")
  (Variables|Default|SetInputEnable true)
  (Variables|Default|SetAction1Pressed false)
  (Variables|Default|SetUseCustomInput false)
  (Variables|Default|SetJumpPressed false)
  (Variables|Default|SetCameraEnable true)
  (Variables|Default|SetTransitionInProgress false)
  (Variables|Default|SetIsJumpEnabled true)
  ;;[1 1 1] Find any gameplay Objects and update overlaps
  (CallFunction|TrytoFindOverlappedObjects)
  (CallFunction|UpdatePlayerRotation))

(event EventTick
  (params (DeltaSeconds :type Float%20%28single-precision%29))
  (bind _velocity (CallFunction|GetVelocity))
  (bind _starttransition (Variables|Default|GetStartTransition))
  (bind _targettransition (Variables|Default|GetTargetTransition))
  ;[1 0.03818 0] Tick
  ;[1 1 1] Calculate common values
  (bind _output_get (Variables|Default|SetIsMoving (>= (Math|Vector|VectorLength (Math|Vector|MakeVector (.x _velocity) (.y _velocity) 0.0)) 1.0)))
  (if _output_get
    (Variables|Default|SetMovementDirection (.yaw (Math|Rotator|Delta(Rotator) (Math|Conversions|RotationFromXVector (CallFunction|GetVelocity)) (Variables|Default|GetPlayerRotation)))))
  (Variables|Default|SetLookingRotation (Pawn|GetControlRotation (Variables|Default|GetPlayerCharacter) :!class /Script/Engine.Pawn))
  (Utilities|FlowControl|Sequence
    (:then_0
      ;[0.2747 1 0.2543] Tick. Uses for Transition
      (if (Variables|Default|GetTransitionInProgress)
        (Variables|Default|SetBlendTime (Math|Float|Clamp(Float) (+ (Variables|Default|GetBlendTime) (* (Utilities|Time|GetWorldDeltaSeconds) (Variables|APCController|GetTransitionSpeed)))))
        (Transformation|SetActorLocationAndRotation (Variables|Default|GetPlayerCharacter) (Math|Interpolation|Ease "EaseInOut" (Variables|Default|GetBlendTime) (.location _starttransition) (.location _targettransition) 2.0) (Math|Rotator|Lerp(Rotator) (.rotation _starttransition) (.rotation _targettransition) (Variables|Default|GetBlendTime) true) false true)
        (if (>= (Variables|Default|GetBlendTime) 1.0)
          (if (not (Variables|Default|GetUnequipInProgress))
            (Variables|Default|SetTransitionInProgress false)
            (CallFunction|FinishActorTransition)))))))

(event EventSetMaxWalkSpeedBPI
  (params (MaxWalkSpeed :type Float%20%28single-precision%29))
  ;[0 0.531 1] Interface events
  (Variables|/Script/Engine.CharacterMovementComponent|SetMaxWalkSpeed (Variables|Default|GetCharacter_MovementComp) MaxWalkSpeed))

(event EventRestoreWalkSpeedBPI
  ;[0 0.531 1] Interface events
  (Variables|/Script/Engine.CharacterMovementComponent|SetMaxWalkSpeed (Variables|Default|GetCharacter_MovementComp) (Variables|Default|GetDefaultWalkSpeed)))

(event EventSetUseCustomInputBPI
  (params (UseCustomInput :type Boolean))
  ;[0 0.531 1] Interface events
  (Variables|Default|SetUseCustomInput UseCustomInput)
  ;;[0.4895 0.9901 1] Reset previous values
  (Variables|Default|SetCustomForwardAxis 0.0)
  (Variables|Default|SetCustomRightAxis 0.0)
  (Variables|Default|SetCustomForwardVector "0, 0, 0")
  (Variables|Default|SetCustomRightVector "0, 0, 0"))

(event EventAddCustomForwardMovementBPI
  (params (AxisValue :type Float%20%28single-precision%29) (ForwardVector :type Vector :default "0, 0, 0"))
  ;[0 0.531 1] Interface events
  (Variables|Default|SetCustomForwardAxis AxisValue)
  (Variables|Default|SetCustomForwardVector ForwardVector))

(event EventAddCustomRightMovementBPI
  (params (AxisValue :type Float%20%28single-precision%29) (RightVector :type Vector :default "0, 0, 0"))
  ;[0 0.531 1] Interface events
  (Variables|Default|SetCustomRightAxis AxisValue)
  (Variables|Default|SetCustomRightVector RightVector))

(event EventOrientPlayertoMovementBPI
  (params (OrientToMovement :type Boolean))
  ;[0 0.531 1] Interface events
  (Variables|/Script/Engine.CharacterMovementComponent|SetbOrientRotationToMovement (Variables|Default|GetCharacter_MovementComp) OrientToMovement))

(event EventSetMovementModeBPI
  (params (Mode :type EMovementMode%20Enum :default "MOVE_None"))
  ;[0 0.531 1] Interface events
  (Pawn|Components|CharacterMovement|SetMovementMode (Variables|Default|GetCharacter_MovementComp) Mode 0))

(event EventSetCapsuleRadiusBPI
  (params (CapsuleRadius :type Float%20%28single-precision%29))
  ;[0 0.531 1] Interface events
  (Components|Capsule|SetCapsuleRadius (Variables|Default|GetCharacter_Capsule) CapsuleRadius true))

(event EventClearOverlappedObjectsBPI
  ;[1 1 1] Immediately reset overlapped objects array
  (Utilities|Array|Clear (Variables|Default|GetOverlappedObjects))
  (Variables|Default|SetCurrentObjectType "NewEnumerator1")
  (Variables|Default|SetCurrentObjectActorPtr 0))

(event EventStartTransitiontoTargetBPI
  (params (Transform :type Transform))
  (bind (_location _rotation) (Math|Transform|BreakTransform Transform))
  (bind _character_capsule (Variables|Default|GetCharacter_Capsule))
  (bind _playercharacter (Variables|Default|GetPlayerCharacter))
  (bind _currentobjectactorptr (Variables|Default|GetCurrentObjectActorPtr))
  (bind (_x _y) (Math|Vector|BreakVector _location))
  (bind _capsulehalfheight (Variables|/Script/Engine.CapsuleComponent|GetCapsuleHalfHeight _character_capsule))
  ;[1 1 1] Transition of player actor to destination location
  (bind _actorstoignore (CallFunction|GetActorstoIngnoreBPI))
  ;;[1 1 1] Add Z offset for target point location depending of floor normal
  (bind (_flooroffsetz _impactlocation) (CallFunction|LIBGetFloorOffsetZ _location (Transformation|GetActorUpVector (Variables|Default|GetPlayerCharacter)) _capsulehalfheight (Variables|/Script/Engine.CapsuleComponent|GetCapsuleRadius _character_capsule) _actorstoignore))
  (Variables|Default|SetTargetTransition (Math|Transform|MakeTransform (Math|Vector|MakeVector _x _y (+ _flooroffsetz (.z _impactlocation) _capsulehalfheight)) _rotation "1,1,1"))
  (Variables|Default|SetInputEnable false)
  (if (and (<= (Math|Vector|VectorLength (- _location (Transformation|GetActorLocation _playercharacter))) 1e+01) (<= (Math|Float|Absolute(Float) (.yaw (Math|Rotator|Delta(Rotator) (Transformation|GetActorRotation _playercharacter) _rotation))) 2.0))
    (Transformation|SetActorLocationAndRotation (Variables|Default|GetPlayerCharacter) (.location (Variables|Default|GetTargetTransition)) (.rotation (Variables|Default|GetTargetTransition)))
    (Utilities|IsValid _currentobjectactorptr
      (:Is%20Valid
        (Class|BPIObjectControls|TransitionCompleteBPI(Message) _currentobjectactorptr (Variables|Default|GetPlayerCharacter)))
      (:Is%20Not%20Valid
        _))
    (Variables|Default|SetInputEnable true)
    (else
      (Variables|Default|SetStartTransition (Transformation|GetWorldTransform (Variables|Default|GetCharacter_Capsule)))
      (Variables|Default|SetBlendTime 0.0)
      (Variables|Default|SetTransitionInProgress true))))

(event EventSetJumpEnabledBPI
  (params (EnableJump :type Boolean))
  ;[0 0.531 1] Interface events
  (Variables|Default|SetIsJumpEnabled EnableJump))

(event EventSetFlyingParametersBPI
  (params (MaxFlySpeed :type Float%20%28single-precision%29) (BrakingDecelerationFlying :type Float%20%28single-precision%29))
  (bind _character_movementcomp (Variables|Default|GetCharacter_MovementComp))
  ;[0 0.531 1] Interface events
  (Variables|/Script/Engine.CharacterMovementComponent|SetMaxFlySpeed _character_movementcomp MaxFlySpeed)
  (Variables|/Script/Engine.CharacterMovementComponent|SetBrakingDecelerationFlying _character_movementcomp BrakingDecelerationFlying))

(event EventSetCapsuleHalfHeightBPI
  (params (CapsuleHalfHeight :type Float%20%28single-precision%29))
  ;[0 0.531 1] Interface events
  (Components|Capsule|SetCapsuleHalfHeight (Variables|Default|GetCharacter_Capsule) CapsuleHalfHeight true))

(event EventForceJumpBPI
  ;[1 1 1] JUMP, Action 1 events
  (Character|Jump (Variables|Default|GetPlayerCharacter))
  (Variables|Default|SetAction1Pressed false)
  (Variables|Default|SetJumpPressed false))

(event EventSetPlayerCollisionResponsetoChannelBPI
  (params (Channel :type ECollisionChannel%20Enum :default "ECC_WorldStatic") (Response :type ECollisionResponse%20Enum :default "ECR_Ignore"))
  ;[0 0.531 1] Interface events
  (Collision|SetCollisionResponsetoChannel (Variables|Default|GetCharacter_Capsule) Channel Response))

(event EventRemoveOverlappedObjectBPI
  (params (Actor :type Actor%20Object%20Reference))
  ;[1 1 1] Remove overlaped object
  (if (Utilities|IsValid Actor)
    (Utilities|Array|RemoveItem (Variables|Default|GetOverlappedObjects) Actor)
    (if (== (Variables|Default|GetCurrentObjectActorPtr) Actor)
      (Variables|Default|SetCurrentObjectActorPtr 0)
      (Variables|Default|SetCurrentObjectType "NewEnumerator1"))
    (else
      (CallFunction|LIBDebugPrint "Error: Attempt to remove object. Actor is not valid!" "(R=1.000000,G=0.000000,B=0.000000,A=1.000000)" 4.0))))

(event EventAddOverlappedObjectBPI
  (params (Actor :type Actor%20Object%20Reference))
  ;[1 1 1] Add overlapped object into array
  (Utilities|Array|AddUnique (Variables|Default|GetOverlappedObjects) Actor))

(event EventSetonVerticalLadderBPI
  (params (OnLadder :type Boolean))
  ;[0 0.531 1] Interface events
  (Variables|Default|SetOnLadder OnLadder))

(event EventPlayAnimMontageBPI
  (params (Montage :type Anim%20Montage%20Object%20Reference) (Instigator :type Actor%20Object%20Reference) (PlayRate :type Float%20%28single-precision%29) (StartPosition :type Float%20%28single-precision%29))
  ;[1 1 1] Play specified Anim Montage
  (Variables|Default|SetAnimMontageInProgress true)
  (Animation|Montage|PlayMontage (Variables|Default|GetCharacter_SkeletalMesh) Montage PlayRate StartPosition
    (:OnCompleted
      (Variables|Default|SetAnimMontageInProgress false)
      (if (Utilities|DoesObjectImplementInterface Instigator "/Game/RisingSignal/Core/InteractLadders/BluePrints/Core/BPI_ObjectControls.BPI_ObjectControls_C")
        (Class|BPIObjectControls|OnMontageCompletedBPI(Message) Instigator (Variables|Default|GetPlayerCharacter))))))

(event EventSimulateActionBPI
  (params (ActionOne :type Boolean))
  (bind _playercharacter (Variables|Default|GetPlayerCharacter))
  ;[1 1 1] JUMP, Action 1 events
  (if ActionOne
    (Variables|Default|SetAction1Pressed true)
    (if (> (Utilities|Array|Length (Variables|Default|GetOverlappedObjects)) 0)
      _
      (else
        (CallFunction|TrytoFindOverlappedObjects)))
    (bind (_actor _type) (CallFunction|GetOverlappedObject))
    (if (Utilities|Enum|NotEqual(Enum) _type "NewEnumerator1")
      (Variables|Default|SetCurrentObjectActorPtr _actor)
      (Variables|Default|SetCurrentObjectType _type)
      (if (Variables|Default|GetAction1Pressed)
        (Class|BPIObjectControls|ActionOneBPI(Message) (Variables|Default|GetCurrentObjectActorPtr) _playercharacter)
        (Variables|Default|SetAction1Pressed false :!label _label)
        (Variables|Default|SetJumpPressed false)
        (else
          (if (Variables|Default|GetJumpPressed) :!label _label_2
            (if (Utilities|Enum|Equal(Enum) (Variables|Default|GetCurrentObjectType) "NewEnumerator3")
              (goto _label)
              (else
                (Character|Jump _playercharacter)
                (goto _label))))))
      (else
        (Variables|Default|SetCurrentObjectActorPtr 0)
        (Variables|Default|SetCurrentObjectType "NewEnumerator1")
        (goto _label_2)))))

(event EventSetEnableInputBPI
  (params (EnableInput :type Boolean))
  ;[0 0.531 1] Interface events
  (Variables|Default|SetInputEnable EnableInput))

(event EventSetEnableCameraBPI
  (params (EnableCamera :type Boolean))
  ;[0 0.531 1] Interface events
  (Variables|Default|SetCameraEnable EnableCamera))

(fn GetOverlappedObject
  (bind _overlappedobjects (Variables|Default|GetOverlappedObjects))
  ;[1 1 1] Try to find closer by angle overlapped object from Player that contain BPI_ObjectCtonrols interface
  (LocalVariables|SetActorIndex -1)
  (if (> (Utilities|Array|Length _overlappedobjects) 0)
    (LocalVariables|SetMinAngle 1e+04)
    (for (_array_element _array_index) _overlappedobjects
      (if (Utilities|DoesObjectImplementInterface _array_element "/Game/RisingSignal/Core/InteractLadders/BluePrints/Core/BPI_ObjectControls.BPI_ObjectControls_C")
        (bind _transform (Class|BPIObjectControls|GetTargetTransform(Message) _array_element))
        (if (< (Class|KismetMathLibrary|DegAcos (Math|Vector|DotProduct (Math|Vector|GetForwardVector (.rotation _transform)) (Math|Vector|GetForwardVector (Variables|Default|GetCharacter_Capsule)))) (LocalVariables|GetMinAngle))
          (LocalVariables|SetMinAngle (Class|KismetMathLibrary|DegAcos (Math|Vector|DotProduct (Math|Vector|GetForwardVector (.rotation _transform)) (Math|Vector|GetForwardVector (Variables|Default|GetCharacter_Capsule)))))
          (LocalVariables|SetActorIndex _array_index))))
    (if (>= (LocalVariables|GetActorIndex) 0)
      (bind _objecttype (Class|BPIObjectControls|GetObjectTypeBPI(Message) (Utilities|Array|Get(acopy) (Variables|Default|GetOverlappedObjects) (LocalVariables|GetActorIndex))))
      (return (Utilities|Array|Get(acopy) (Variables|Default|GetOverlappedObjects) (LocalVariables|GetActorIndex)) _objecttype)
      (else
        _)))
  (return 0 "NewEnumerator1"))

(fn TrytoFindCamera
  ;[1 1 1] Try to find Camera component with specified Name.
  (for _array_element (Actor|GetComponentsByClass (Components|GetOwner) "/Script/Engine.CameraComponent")
    (if (Utilities|Enum|Equal(Enum) (Utilities|GetObjectName _array_element) (Variables|APCController|GetMainCameraName))
      (return _array_element)))
  (return 0))

(fn TrytoFindSpringArm
  (bind _returnvalue (Components|GetOwner))
  (bind _returnvalue_2 (Actor|GetComponentbyClass _returnvalue "/Script/Engine.SpringArmComponent"))
  ;[1 1 1] Try to find SpringArm component. Please don't add more than one SpringArm component in to Character!
  (Utilities|IsValid _returnvalue_2
    (:Is%20Valid
      (return _returnvalue_2))
    (:Is%20Not%20Valid
      (return 0))))

(fn GetVelocity
  (return (Transformation|GetVelocity (Components|GetOwner))))

(fn CalcRotationRate
  (params (SlowSpeed :type Float%20%28single-precision%29) (SlowSpeedRate :type Float%20%28single-precision%29) (FastSpeed :type Float%20%28single-precision%29) (FastSpeedRate :type Float%20%28single-precision%29))
  (bind _velocity (CallFunction|GetVelocity))
  (bind _returnvalue (Math|Vector|MakeVector (.x _velocity) (.y _velocity) 0.0))
  (bind _returnvalue_2 (Math|Vector|VectorLength _returnvalue))
  ;[1 1 1] Dynamically set Rotation Rate based on characters movement speed. Supports 2 Rotation Rates for differnet speeds. The Rotation Rate Multiplier is used to ramp down rotation rate whenever it is set to 0 (Automatically returns to 1)
  (return (Math|Float|Clamp(Float) (* (select (> _returnvalue_2 SlowSpeed) (Math|Float|MapRangeUnclamped _returnvalue_2 SlowSpeed FastSpeed SlowSpeedRate FastSpeedRate) (Math|Float|MapRangeClamped _returnvalue_2 0.0 SlowSpeed 0.0 SlowSpeedRate)) 1.0) 0.1 15.0)))

(fn AnimGetDirectionBPI
  (return (Variables|Default|GetMovementDirection)))

(fn AnimGetForwardAxisBPI
  ;[1 1 1] Return forward axis value
  (return (Variables|Default|GetForwardAxisValue)))

(fn AnimIsMovingBPI
  (return (Variables|Default|GetIsMoving)))

(fn AnimIsonLadderBPI
  ;[1 1 1] Return is on the Vertical Ladder
  (return (Variables|Default|GetOnLadder)))

(fn AnimIsPlayingRecoilBPI
  (return (Variables|Default|GetPlayRecoilAnim)))

(fn CanbeUsedBPI
  ;[1 1 1] Return is box attached to Player
  (return (and (not (Variables|Default|GetIsPushingBoxAttached)) (not (Variables|Default|GetAimMode)))))

(fn GetActorstoIngnoreBPI
  (bind _tempactorsarray (LocalVariables|GetTempActorsArray))
  ;[1 1 1] Add your own spcified actors here if required to be ignored
  (for _array_element 0
    (Utilities|Array|Add _tempactorsarray _array_element))
  (Utilities|Array|Add _tempactorsarray (Components|GetOwner))
  (return _tempactorsarray))

(fn GetAimRotationandLocationBPI
  (bind _character_camera (Variables|Default|GetCharacter_Camera))
  (bind _returnvalue (Math|Vector|GetForwardVector _character_camera))
  (return _returnvalue (+ (* _returnvalue 0.0) (Transformation|GetWorldLocation _character_camera))))

(fn GetCapsuleHalfHeightBPI
  ;[1 1 1] Return capsule half height
  (return (Variables|/Script/Engine.CapsuleComponent|GetCapsuleHalfHeight (Variables|Default|GetCharacter_Capsule))))

(fn GetCapsuleRadiusBPI
  ;[1 1 1] Return capsule radius
  (return (Variables|/Script/Engine.CapsuleComponent|GetCapsuleRadius (Variables|Default|GetCharacter_Capsule))))

(fn GetCapsuleTransformBPI
  ;[1 1 1] Return capsule transform
  (return (Transformation|GetWorldTransform (Variables|Default|GetCharacter_Capsule))))

(fn GetCharacterControllerBPI
  ;[1 1 1] Retun Player Controller of Character
  (return (Game|GetPlayerController 0)))

(fn GetCharacterControlRotationBPI
  ;[1 1 1] Retun Controller Rotator
  (return (Pawn|GetControlRotation (Variables|Default|GetPlayerCharacter) :!class /Script/Engine.Pawn)))

(fn GetFlyingParametersBPI
  (bind _character_movementcomp (Variables|Default|GetCharacter_MovementComp))
  (return (Variables|/Script/Engine.CharacterMovementComponent|GetMaxFlySpeed _character_movementcomp) (Variables|/Script/Engine.CharacterMovementComponent|GetBrakingDecelerationFlying _character_movementcomp)))

(fn HasOverlappedObjectBPI
  ;[1 1 1] Check is any object is overlapped
  (return (> (Utilities|Array|Length (Variables|Default|GetOverlappedObjects)) 0)))