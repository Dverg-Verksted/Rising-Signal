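; BP_ClimbingWall is a climbable wall interactable that supplies climbing settings and tracks whether climbing is active.
; On BeginPlay it copies its climbing speed and wall distance onto the BP_RSGamePlayer character.
; Overlapping its ClimbingCollision volume sets its IsClimbing flag, without filtering the overlapping actor.
; Ending the overlap clears the flag after a short delay.
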(event OnComponentBeginOverlap(ClimbingCollision)
  (params (OverlappedComponent :type Primitive%20Component%20Object%20Reference) (OtherActor :type Actor%20Object%20Reference) (OtherComp :type Primitive%20Component%20Object%20Reference) (OtherBodyIndex :type Integer) (bFromSweep :type Boolean) (SweepResult :type Hit%20Result%20Structure%20%28by%20ref%29))
  ;[1 1 1] Активация взаимодействия с залазом
  (Variables|Default|SetIsClimbing true))

(event OnComponentEndOverlap(ClimbingCollision)
  (params (OverlappedComponent :type Primitive%20Component%20Object%20Reference) (OtherActor :type Actor%20Object%20Reference) (OtherComp :type Primitive%20Component%20Object%20Reference) (OtherBodyIndex :type Integer))
  ;[1 1 1] Дизактивация взаимодействия с залазом
  (Utilities|FlowControl|Delay 1.2)
  (Variables|Default|SetIsClimbing false))

(event EventBeginPlay
  (bind _asbp_rsgame_player (Utilities|Casting|CastToBP_RSGamePlayer (Game|GetPlayerCharacter 0)))
  (Variables|/Game/RisingSignal/Core/Player/BP_RSGamePlayer.BP_RSGamePlayer_C|SetClimbingSpeed _asbp_rsgame_player (Variables|Default|GetClimbingSpeed))
  (Variables|/Game/RisingSignal/Core/Player/BP_RSGamePlayer.BP_RSGamePlayer_C|SetWallDistance _asbp_rsgame_player (Variables|Default|GetWallDistance)))

(event Collision|EventActorBeginOverlap
  (params (OtherActor :type Actor%20Object%20Reference)))

(event EventTick
  (params (DeltaSeconds :type Float%20%28single-precision%29)))

(fn ConstructionScript)