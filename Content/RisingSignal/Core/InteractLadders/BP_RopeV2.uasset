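; BP_RopeV2 is a rope the player can grab and swing on.
; Overlapping its Capsule checks the other actor via a player message call and, if it passes, sends it GrabRopeMessage with the rope.
; AddSwingingForce pushes CableEnd with a scaled, inverted acceleration-change force.
; To limit swinging, the force is skipped while CableEnd's vertical drop below the actor origin lies within a fixed band.
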(event OnComponentBeginOverlap(Capsule)
  (params (OverlappedComponent :type Primitive%20Component%20Object%20Reference) (OtherActor :type Actor%20Object%20Reference) (OtherComp :type Primitive%20Component%20Object%20Reference) (OtherBodyIndex :type Integer) (bFromSweep :type Boolean) (SweepResult :type Hit%20Result%20Structure%20%28by%20ref%29))
  ;[1 1 1] Захват верёвки
  (bind _yes_no (Class|BPIPlayer|IsPlayer(Message) OtherActor))
  (if _yes_no
    (Class|BPIPlayer|GrabRope(Message) OtherActor self)))

(event Custom|AddSwingingForce
  (params (SwingForce :type Vector))
  (bind _returnvalue (Transformation|GetActorLocation))
  (bind _cableend (Variables|Default|GetCableEnd))
  (bind _returnvalue_2 (Transformation|GetWorldLocation _cableend))
  (bind _returnvalue_3 (- (.z _returnvalue) (.z _returnvalue_2)))
  ;[1 1 1] Добавление силы для раскачивания верёвки
  (if (not (and (< _returnvalue_3 9.9e+02) (> _returnvalue_3 5e+02)))
    (Physics|AddForce (Variables|Default|GetCableEnd) (* SwingForce -2.5e+02) "None" true)))

(event EventBeginPlay)

(event Collision|EventActorBeginOverlap
  (params (OtherActor :type Actor%20Object%20Reference)))

(event EventTick
  (params (DeltaSeconds :type Float%20%28single-precision%29)))

(fn ConstructionScript)