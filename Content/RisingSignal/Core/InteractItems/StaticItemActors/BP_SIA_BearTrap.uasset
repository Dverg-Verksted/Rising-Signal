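; BP_SIA_BearTrap is a single-use bear trap actor that damages and briefly immobilizes the player.
; When a BP_BasePlayer capsule overlaps its sphere collision while active, it deactivates, stops the player's movement, disables input and applies damage.
; It also rescales the trap mesh, spawns a blood Niagara effect and shows a "Trapped" HUD notification.
; A one-shot timer restores player input after a configurable duration.
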(event OnComponentBeginOverlap(SphereCollision)
  (params (OverlappedComponent :type Primitive%20Component%20Object%20Reference) (OtherActor :type Actor%20Object%20Reference) (OtherComp :type Primitive%20Component%20Object%20Reference) (OtherBodyIndex :type Integer) (bFromSweep :type Boolean) (SweepResult :type Hit%20Result%20Structure%20%28by%20ref%29))
  (if (Variables|Default|GetbActive)
    (bind _ascapsule_collision (Utilities|Casting|CastToCapsuleComponent OtherComp))
    (bind _asbp_base_player (Utilities|Casting|CastToBP_BasePlayer (Components|GetOwner _ascapsule_collision)))
    (Variables|Default|SetPlayerRef _asbp_base_player)
    (Variables|Default|SetbActive false)
    (Components|Movement|StopMovementImmediately (Variables|/Script/Engine.Character|GetCharacterMovement (Variables|Default|GetPlayerRef)))
    (Input|DisableInput (Variables|Default|GetPlayerRef) (Variables|/Script/RisingSignal.RSBaseCharacter|GetGamePlayerController (Variables|Default|GetPlayerRef)))
    (Game|Damage|ApplyDamage (Variables|Default|GetPlayerRef) (Variables|Default|GetDamageAmount) 0 0)
    (Utilities|Time|SetTimerbyEvent (delegate Custom|RestartInput) (Variables|Default|GetDisableMovementFor))
    (Transformation|SetWorldScale3D (Variables|Default|GetBearTrapMesh) "0.300000,0.300000,0.300000")
    (Niagara|SpawnSystematLocation "/Game/RisingSignal/Assets/Marketplace/AI/Wolf/VFX/NS_BiteBlood.NS_BiteBlood" (Transformation|GetActorLocation self))
    (Default|ShowNotification (Variables|/Game/RisingSignal/Core/HUD/UI_UserHUD/Widgets/WBP_PlayerInterface.WBP_PlayerInterface_C|GetWBP_Notification (Variables|/Game/RisingSignal/Core/Player/BP_PlayerHUD.BP_PlayerHUD_C|GetPlayerInterfaceRef (Variables|/Game/RisingSignal/Core/Player/BP_BasePlayer.BP_BasePlayer_C|GetPlayer%20HUDRef (Variables|Default|GetPlayerRef)))) "Trapped" true 2.0)))

(event Custom|RestartInput
  (Input|EnableInput (Variables|Default|GetPlayerRef) (Variables|/Script/RisingSignal.RSBaseCharacter|GetGamePlayerController (Variables|Default|GetPlayerRef))))

(event EventBeginPlay)

(event EventTick
  (params (DeltaSeconds :type Float%20%28single-precision%29)))

(fn ConstructionScript)