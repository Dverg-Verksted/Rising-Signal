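; Test player character for the RisingSignal user HUD, inventory and action bar.
; BeginPlay creates WBP_HUD and binds RSInventory events to a debug print; I or ClickedToClose toggles inventory, cursor and input mode through one FlipFlop.
; Keys 1-4 use occupied action bar slots through the player controller, and PickUpItem passes pickup data table rows to RSInventory.
; A/D provide rough horizontal movement by re-triggering MoveComponentTo on the capsule while held.
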(event Custom|ClickedToClose
  (bind _hudref (Variables|Default|GetHUDRef))
  (bind _controllerref (Variables|Default|GetControllerRef))
  (bind _wbp_inventory (Variables|/Game/RisingSignal/Core/HUD/UI_UserHUD/Widgets/WBP_HUD.WBP_HUD_C|GetWBP_Inventory _hudref))
  ;[1 1 1] Used to toggle inventory menu
  (Utilities|FlowControl|FlipFlop
    (:A
      (Variables|/Game/RisingSignal/Core/HUD/UI_UserHUD/Widgets/WBP_Inventory.WBP_Inventory_C|SetInventoryVisible _wbp_inventory "Visible")
      (Input|SetInputModeGameandUI _controllerref (Variables|Default|GetHUDRef) "LockInFullscreen" true)
      (Variables|/Script/Engine.PlayerController|SetbShowMouseCursor _controllerref true)
      ;;[1 0.9667 0.4135] Can be used for disable movement, but you should to use state and enum for this control
      (Variables|Default|SetMenuOpen? true))
    (:B
      (Variables|/Game/RisingSignal/Core/HUD/UI_UserHUD/Widgets/WBP_Inventory.WBP_Inventory_C|SetInventoryVisible _wbp_inventory "Hidden")
      (Input|SetInputModeGameOnly _controllerref)
      (Variables|/Script/Engine.PlayerController|SetbShowMouseCursor _controllerref false)
      (Variables|Default|SetMenuOpen? false))))

(event Custom|OnInventoryActions
  (params (IventoryEvent :type EInventoryEvent%20Enum :default "Remove") (FirstItem :type Inventory%20Item%20Structure))
  (Development|PrintString (Class|RSInventoryComponent|ToString FirstItem)))

(event EventBeginPlay
  (bind _asbp_rsgame_player_controller (Utilities|Casting|CastToBP_RSGamePlayerController (Game|GetPlayerController 0)))
  (bind _output_get (Variables|Default|SetControllerRef _asbp_rsgame_player_controller))
  (bind _returnvalue (UserInterface|CreateWidget "/Game/RisingSignal/Core/HUD/UI_UserHUD/Widgets/WBP_HUD.WBP_HUD_C" _output_get))
  (bind _output_get_2 (Variables|Default|SetHUDRef _returnvalue))
  (UserInterface|Viewport|AddtoViewport _output_get_2 0)
  (EventDispatchers|AssignOnInventoryEvent (Variables|Default|GetRSInventory) (delegate Custom|OnInventoryActions)))

(event Collision|EventActorBeginOverlap
  (params (OtherActor :type Actor%20Object%20Reference)))

(event EventTick
  (params (DeltaSeconds :type Float%20%28single-precision%29)))

(event Input|KeyboardEvents|1
  (params (Key :type Key%20Structure :default "None"))
  ;[1 1 1] Перенести в контроллер, на всякий случай кинул тут, мало ли там цифры за что то отвечают
  (:Pressed
    (CallFunction|UsedActionBar)))

(event Input|KeyboardEvents|2
  (params (Key :type Key%20Structure :default "None"))
  ;[1 1 1] Перенести в контроллер, на всякий случай кинул тут, мало ли там цифры за что то отвечают
  (:Pressed
    (CallFunction|UsedActionBar 1)))

(event Input|KeyboardEvents|3
  (params (Key :type Key%20Structure :default "None"))
  ;[1 1 1] Перенести в контроллер, на всякий случай кинул тут, мало ли там цифры за что то отвечают
  (:Pressed
    (CallFunction|UsedActionBar 2)))

(event Input|KeyboardEvents|4
  (params (Key :type Key%20Structure :default "None"))
  ;[1 1 1] Перенести в контроллер, на всякий случай кинул тут, мало ли там цифры за что то отвечают
  (:Pressed
    (CallFunction|UsedActionBar 3)))

(event Input|KeyboardEvents|D
  (params (Key :type Key%20Structure :default "None"))
  (bind _returnvalue (Transformation|GetActorLocation))
  ;[1 1 1] Add some Hor Movement
  (:Pressed
    (Variables|Default|SetisMove true)
    (Variables|Default|SetMovementOrient -1.0)
    (Components|MoveComponentTo (Variables|Collision|GetCapsuleComponent) (Math|Vector|MakeVector (+ (.x _returnvalue) (* (Variables|Default|GetMovementOrient) 75.0)) (.y _returnvalue) (.z _returnvalue)) "0, 0, 0" false false 0.2 false :!label _label)
    (if (Variables|Default|GetisMove)
      (goto _label)
      (else
        (goto _label Stop))))
  (:Released
    (Variables|Default|SetisMove false)))

(event Input|KeyboardEvents|A
  (params (Key :type Key%20Structure :default "None"))
  (bind _returnvalue (Transformation|GetActorLocation))
  ;[1 1 1] Add some Hor Movement
  (:Pressed
    (Variables|Default|SetisMove true)
    (Variables|Default|SetMovementOrient 1.0)
    (Components|MoveComponentTo (Variables|Collision|GetCapsuleComponent) (Math|Vector|MakeVector (+ (.x _returnvalue) (* (Variables|Default|GetMovementOrient) 75.0)) (.y _returnvalue) (.z _returnvalue)) "0, 0, 0" false false 0.2 false :!label _label)
    (if (Variables|Default|GetisMove)
      (goto _label)
      (else
        (goto _label Stop))))
  (:Released
    (Variables|Default|SetisMove false)))

(event Input|KeyboardEvents|I
  (params (Key :type Key%20Structure :default "None"))
  (bind _hudref (Variables|Default|GetHUDRef))
  (bind _controllerref (Variables|Default|GetControllerRef))
  (bind _wbp_inventory (Variables|/Game/RisingSignal/Core/HUD/UI_UserHUD/Widgets/WBP_HUD.WBP_HUD_C|GetWBP_Inventory _hudref))
  ;[1 1 1] Used to toggle inventory menu
  (:Pressed
    (Utilities|FlowControl|FlipFlop
      (:A
        (Variables|/Game/RisingSignal/Core/HUD/UI_UserHUD/Widgets/WBP_Inventory.WBP_Inventory_C|SetInventoryVisible _wbp_inventory "Visible")
        (Input|SetInputModeGameandUI _controllerref (Variables|Default|GetHUDRef) "LockInFullscreen" true)
        (Variables|/Script/Engine.PlayerController|SetbShowMouseCursor _controllerref true)
        ;;[1 0.9667 0.4135] Can be used for disable movement, but you should to use state and enum for this control
        (Variables|Default|SetMenuOpen? true))
      (:B
        (Variables|/Game/RisingSignal/Core/HUD/UI_UserHUD/Widgets/WBP_Inventory.WBP_Inventory_C|SetInventoryVisible _wbp_inventory "Hidden")
        (Input|SetInputModeGameOnly _controllerref)
        (Variables|/Script/Engine.PlayerController|SetbShowMouseCursor _controllerref false)
        (Variables|Default|SetMenuOpen? false)))))

(fn ConstructionScript)

(fn UsedActionBar
  (params (Slot :type Integer))
  (Utilities|IsValid (Utilities|Array|Get(acopy) (Variables|/Game/RisingSignal/Core/HUD/UI_UserHUD/Widgets/WBP_ActionBar.WBP_ActionBar_C|GetActionButtons (Variables|/Game/RisingSignal/Core/HUD/UI_UserHUD/Widgets/WBP_HUD.WBP_HUD_C|GetWBP_ActionBar (Variables|Default|GetHUDRef))) Slot)
    (:Is%20Valid
      (Default|UseItemEvent (Variables|Default|GetControllerRef) Slot))))

(fn PickUpItem
  (params (Item%20to%20Pickup :type Object%20Object%20Reference))
  (bind _asbp_pick_up (Utilities|Casting|CastToBP_PickUp Item%20to%20Pickup))
  (bind _returnvalue (Utilities|GetDataTableRow "/Game/RisingSignal/Core/HUD/UI_UserHUD/Blueprints/DT_TestInventoryItems.DT_TestInventoryItems" (Utilities|String|StringToName (Variables|/Game/RisingSignal/Core/HUD/UI_UserHUD/Blueprints/BP_PickUp.BP_PickUp_C|GetRowName _asbp_pick_up)))
    (:then
      (Class|RSInventoryComponent|ActionItem (Variables|Default|GetRSInventory) _returnvalue (Utilities|Struct|MakeInventoryItem 0 -1) "Motion"))))