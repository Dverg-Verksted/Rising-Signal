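; BP_PlayerTestHUD is a test player HUD actor that owns the main on-screen widget and switches between gameplay and inventory views.
; On BeginPlay it creates WBP_HUD, adds it to the viewport and caches the ALS player controller.
; ShowInventory and HideInventory events toggle the inventory's visibility variable, show or collapse user stats inversely, and switch input mode and mouse cursor to match.
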(event Custom|ShowInventory
  (bind _controllerref (Variables|Default|GetControllerRef))
  (Variables|/Game/RisingSignal/Core/HUD/UI_UserHUD/Widgets/WBP_Inventory.WBP_Inventory_C|SetInventoryVisible (Variables|/Game/RisingSignal/Core/HUD/UI_UserHUD/Widgets/WBP_HUD.WBP_HUD_C|GetWBP_Inventory (Variables|Default|GetHUDRef)) "Visible")
  (Widget|SetVisibility (Variables|/Game/RisingSignal/Core/HUD/UI_UserHUD/Widgets/WBP_HUD.WBP_HUD_C|GetWBP_UserStats (Variables|Default|GetHUDRef)) "Collapsed")
  (Input|SetInputModeGameandUI _controllerref (Variables|Default|GetHUDRef) "LockInFullscreen" true)
  (Variables|/Script/Engine.PlayerController|SetbShowMouseCursor _controllerref true))

(event Custom|HideInventory
  (bind _controllerref (Variables|Default|GetControllerRef))
  (Variables|/Game/RisingSignal/Core/HUD/UI_UserHUD/Widgets/WBP_Inventory.WBP_Inventory_C|SetInventoryVisible (Variables|/Game/RisingSignal/Core/HUD/UI_UserHUD/Widgets/WBP_HUD.WBP_HUD_C|GetWBP_Inventory (Variables|Default|GetHUDRef)) "Hidden")
  (Widget|SetVisibility (Variables|/Game/RisingSignal/Core/HUD/UI_UserHUD/Widgets/WBP_HUD.WBP_HUD_C|GetWBP_UserStats (Variables|Default|GetHUDRef)) "Visible")
  (Input|SetInputModeGameOnly _controllerref)
  (Variables|/Script/Engine.PlayerController|SetbShowMouseCursor _controllerref false))

(event EventBeginPlay
  (bind _returnvalue (UserInterface|CreateWidget "/Game/RisingSignal/Core/HUD/UI_UserHUD/Widgets/WBP_HUD.WBP_HUD_C"))
  (bind _output_get (Variables|Default|SetHudRef _returnvalue))
  (UserInterface|Viewport|AddtoViewport _output_get 0)
  (bind _asbp_als_player_controller (Utilities|Casting|CastToBP_Als_PlayerController (Game|GetPlayerController 0)))
  (Variables|Default|SetControllerRef _asbp_als_player_controller))

(fn ConstructionScript)