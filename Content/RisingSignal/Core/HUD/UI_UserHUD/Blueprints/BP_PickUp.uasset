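; BP_PickUp is a world item that the test player character picks up by walking into its trigger.
; BeginPlay caches the player controller and character, though only the character reference is used here.
; On overlap it passes itself to the character's PickUpItem, then hides and disables collision instead of destroying itself, without checking whether the pickup succeeded.
; DoStuff is a placeholder event that prints a debug string.
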(event OnComponentBeginOverlap(Trigger)
  (params (OverlappedComponent :type Primitive%20Component%20Object%20Reference) (OtherActor :type Actor%20Object%20Reference) (OtherComp :type Primitive%20Component%20Object%20Reference) (OtherBodyIndex :type Integer) (bFromSweep :type Boolean) (SweepResult :type Hit%20Result%20Structure%20%28by%20ref%29))
  ;[1 1 1] Pick up the item, if has free sapce
  (Utilities|Casting|CastToBP_TestPlayerCharacter OtherActor)
  (Default|PickUpItem (Variables|Default|GetCharacterRef) self)
  (Rendering|SetActorHiddenInGame true)
  (Collision|SetActorEnableCollision false))

(event Custom|DoStuff
  (Development|PrintString "Do cool stuff"))

(event EventBeginPlay
  ;[1 1 1] Get References
  (bind _asbp_rsgame_player_controller (Utilities|Casting|CastToBP_RSGamePlayerController (Game|GetPlayerController 0)))
  (Variables|Default|SetControllerRef _asbp_rsgame_player_controller)
  (bind _asbp_test_player_character (Utilities|Casting|CastToBP_TestPlayerCharacter (Game|GetPlayerCharacter 0)))
  (Variables|Default|SetCharacterRef _asbp_test_player_character))

(event Collision|EventActorBeginOverlap
  (params (OtherActor :type Actor%20Object%20Reference)))

(event EventTick
  (params (DeltaSeconds :type Float%20%28single-precision%29)))

(fn ConstructionScript)