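; Test player character for the user HUD and inventory, which creates WBP_HUD on BeginPlay and caches it with the RS game player controller.
; The I key and ClickedToClose share one FlipFlop that toggles inventory visibility, cursor, input mode and MenuOpen.
; Number keys 1-4 check for a valid action bar button, then call UseItemEvent on the controller.
; Debug keys print the inventory check, clear the inventory or apply sideways capsule impulses.
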(event Custom|ClickedToClose
  (bind _hudref (Variables|Default|GetHUDRef))
  (bind _controllerref (Variables|Default|GetControllerRef))
  (bind _wbp_inventorydrag (Variables|/Game/RisingSignal/Core/HUD/UI_UserHUD/WBP_HUD.WBP_HUD_C|GetWBP_InventoryDrag _hudref))
  ;[1 1 1] Used to toggle inventory menu
  (Utilities|FlowControl|FlipFlop
    (:A
      (Variables|/Game/RisingSignal/Core/HUD/UI_UserHUD/WBP_InventoryDrag.WBP_InventoryDrag_C|SetInventoryVisible _wbp_inventorydrag "Visible")
      (Input|SetInputModeGameandUI _controllerref (Variables|Default|GetHUDRef) "LockInFullscreen" true)
      (Variables|/Script/Engine.PlayerController|SetbShowMouseCursor _controllerref true)
      ;;[1 0.9667 0.4135] Can be used for disable movement, but you should to use state and enum for this control
      (Variables|Default|SetMenuOpen? true))
    (:B
      (Variables|/Game/RisingSignal/Core/HUD/UI_UserHUD/WBP_InventoryDrag.WBP_InventoryDrag_C|SetInventoryVisible _wbp_inventorydrag "Hidden")
      (Input|SetInputModeGameOnly _controllerref)
      (Variables|/Script/Engine.PlayerController|SetbShowMouseCursor _controllerref false)
      (Variables|Default|SetMenuOpen? false))))

(event EventBeginPlay
  (bind _asbp_rsgame_player_controller (Utilities|Casting|CastToBP_RSGamePlayerController (Game|GetPlayerController 0)))
  (bind _output_get (Variables|Default|SetControllerRef _asbp_rsgame_player_controller))
  (bind _returnvalue (UserInterface|CreateWidget "/Game/RisingSignal/Core/HUD/UI_UserHUD/WBP_HUD.WBP_HUD_C" _output_get))
  (bind _output_get_2 (Variables|Default|SetHUDRef _returnvalue))
  (UserInterface|Viewport|AddtoViewport _output_get_2 0))

(event Collision|EventActorBeginOverlap
  (params (OtherActor :type Actor%20Object%20Reference)))

(event EventTick
  (params (DeltaSeconds :type Float%20%28single-precision%29)))

(event Input|KeyboardEvents|F
  (params (Key :type Key%20Structure))
  ;[1 1 1] Check is inventory works correct
  (:Pressed
    (bind _bhasspace (Default|InventoryCheck (Variables|Default|GetControllerRef)))
    (Development|PrintString (Utilities|String|ToString(Boolean) _bhasspace))))

(event Input|KeyboardEvents|G
  (params (Key :type Key%20Structure))
  ;[1 1 1] Check is inventory works correct
  (:Pressed
    (Default|ClearInventory (Variables|Default|GetControllerRef))))

(event Input|KeyboardEvents|1
  (params (Key :type Key%20Structure))
  (:Pressed
    (CallFunction|UsedActionBar)))

(event Input|KeyboardEvents|2
  (params (Key :type Key%20Structure))
  (:Pressed
    (CallFunction|UsedActionBar 1)))

(event Input|KeyboardEvents|3
  (params (Key :type Key%20Structure))
  (:Pressed
    (CallFunction|UsedActionBar 2)))

(event Input|KeyboardEvents|4
  (params (Key :type Key%20Structure))
  (:Pressed
    (CallFunction|UsedActionBar 3)))

(event Input|KeyboardEvents|D
  (params (Key :type Key%20Structure))
  ;[1 1 1] Add some Hor Movement
  (:Pressed
    (Physics|AddImpulse (Variables|Collision|GetCapsuleComponent) "-300.000000, 0, 0" "None" true)))

(event Input|KeyboardEvents|A
  (params (Key :type Key%20Structure))
  ;[1 1 1] Add some Hor Movement
  (:Pressed
    (Physics|AddImpulse (Variables|Collision|GetCapsuleComponent) "300.000000, 0, 0" "None" true)))

(event Input|KeyboardEvents|I
  (params (Key :type Key%20Structure))
  (bind _hudref (Variables|Default|GetHUDRef))
  (bind _controllerref (Variables|Default|GetControllerRef))
  (bind _wbp_inventorydrag (Variables|/Game/RisingSignal/Core/HUD/UI_UserHUD/WBP_HUD.WBP_HUD_C|GetWBP_InventoryDrag _hudref))
  ;[1 1 1] Used to toggle inventory menu
  (:Pressed
    (Utilities|FlowControl|FlipFlop
      (:A
        (Variables|/Game/RisingSignal/Core/HUD/UI_UserHUD/WBP_InventoryDrag.WBP_InventoryDrag_C|SetInventoryVisible _wbp_inventorydrag "Visible")
        (Input|SetInputModeGameandUI _controllerref (Variables|Default|GetHUDRef) "LockInFullscreen" true)
        (Variables|/Script/Engine.PlayerController|SetbShowMouseCursor _controllerref true)
        ;;[1 0.9667 0.4135] Can be used for disable movement, but you should to use state and enum for this control
        (Variables|Default|SetMenuOpen? true))
      (:B
        (Variables|/Game/RisingSignal/Core/HUD/UI_UserHUD/WBP_InventoryDrag.WBP_InventoryDrag_C|SetInventoryVisible _wbp_inventorydrag "Hidden")
        (Input|SetInputModeGameOnly _controllerref)
        (Variables|/Script/Engine.PlayerController|SetbShowMouseCursor _controllerref false)
        (Variables|Default|SetMenuOpen? false)))))

(fn ConstructionScript)

(fn UsedActionBar
  (params (Slot :type Integer))
  (Utilities|IsValid (Utilities|Array|Get(acopy) (Variables|/Game/RisingSignal/Core/HUD/UI_UserHUD/WBP_ActionBar.WBP_ActionBar_C|GetActionButtons (Variables|/Game/RisingSignal/Core/HUD/UI_UserHUD/WBP_HUD.WBP_HUD_C|GetWBP_ActionBar (Variables|Default|GetHUDRef))) Slot)
    (:Is%20Valid
      (Default|UseItemEvent (Variables|Default|GetControllerRef) Slot))))